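; Inspectable actor component that gives its owner a display name and a status for inspection.
; On BeginPlay it takes the name from the owner's object name, and GetStatus reports "Dead" when the owner's Bpc_State says so.
; Inspect and UnInspect are empty events; disconnected logic would drive the player controller's main widget and toggle custom depth on item meshes.
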(event `self.ReceiveBeginPlay`
  (set `self.name` (`KismetTextLibrary.Conv_StringToText` (`KismetSystemLibrary.GetObjectName` (`self.GetOwner`)))))

(event `Inspect`)

(event `UnInspect`)

(fn `GetStatus`
  (locals (status :type Name))
  (bind _returnvalue (`Actor.GetComponentByClass` (`self.GetOwner`) "/Game/MMORPG/Buleprint/Characters/State/Bpc_State.Bpc_State_C"))
  (if (and (`KismetSystemLibrary.IsValid` _returnvalue) (`/Game/MMORPG/Buleprint/Characters/State/Bpc_State.IsDead` _returnvalue))
    (set `local.status` "Dead")))
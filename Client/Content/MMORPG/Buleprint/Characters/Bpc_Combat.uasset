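; Combat component for Bp_CharacterBase characters that handles attacks, incoming hits and a combat-status toggle.
; Attack broadcasts the weapon type and plays a fixed double-sword montage, holding attack and hit flags until completion.
; OnHit clears its hit flag and applies fixed damage to the owner.
; The bound damage handler plays a bow hit-reaction montage and subtracts the truncated damage from a Bpc_State stat.
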(event `self.ReceiveBeginPlay`
  (add `Actor.OnTakeAnyDamage` (`self.GetOwner`) (delegate `OnTakeAnyDamage_事件_0`)))

(event `OnTakeAnyDamage_事件_0`
  (params (DamagedActor :type "Actor Object Reference") (Damage :type "Float (double-precision)") (DamageType :type "DamageType Object Reference") (InstigatedBy :type "Controller Object Reference") (DamageCauser :type "Actor Object Reference"))
  (bind _returnvalue (`self.GetOwner`))
  (bind _returnvalue_2 (`Actor.GetComponentByClass` _returnvalue "/Game/MMORPG/Buleprint/Characters/State/Bpc_State.Bpc_State_C"))
  (`|PlayMontage` (`Character.Mesh` (cast `/Game/MMORPG/Buleprint/Characters/Bp_CharacterBase` _returnvalue :!pure true)) "/Game/MMORPG/Buleprint/Characters/Common/Animations/GetHit_BowAnim_Montage.GetHit_BowAnim_Montage"
    (:`then`
      (`/Engine/EditorBlueprintResources/StandardMacros.IsValid` _returnvalue_2
        (:`Is Valid`
          (`/Game/MMORPG/Buleprint/Characters/State/Bpc_State.ModifyStat` _returnvalue_2 "NewEnumerator1" (* (`KismetMathLibrary.FTrunc` Damage) -1)))))))

(event `self.ReceiveEndPlay`
  (params (EndPlayReason :type "EEndPlayReason Enum" :default "Destroyed"))
  (remove `Actor.OnTakeAnyDamage` (`self.GetOwner`) (delegate `OnTakeAnyDamage_事件_0`)))

(event `Attack`
  (bind _weapontype (`self.WeaponType`))
  (bind (_asbp_character_base _bsuccess) (cast `/Game/MMORPG/Buleprint/Characters/Bp_CharacterBase` (`self.GetOwner`) :!pure true))
  (if (`|EnumInequality` _weapontype "NewEnumerator5")
    (if (and _bsuccess (not (`self.isAttack?`)))
      (`self.OnAttack` _weapontype)
      (set `self.isAttack?` true)
      (set `self.isHit?` true)
      (`|PlayMontage` (`Character.Mesh` _asbp_character_base) "/Game/MMORPG/Buleprint/Characters/Common/Animations/NormalAttack01_DoubleSwordAnim_Montage.NormalAttack01_DoubleSwordAnim_Montage"
        (:`OnCompleted`
          (set `self.isAttack?` false)
          (set `self.isHit?` false))))))

(event `OnHit`
  (params (instigator :type "Controller Object Reference") (Causer :type "Actor Object Reference"))
  (set `self.isHit?` false)
  (`GameplayStatics.ApplyDamage` (`self.GetOwner`) 10.0 instigator Causer))

(fn `SwitchCombatStatus`
  (bind _output_get (set `self.isCombat?` (not (`self.isCombat?`))))
  (`self.OnStatuChange` _output_get))
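; Player character component that manages modular outfit parts by swapping skeletal meshes per dress slot.
; On BeginPlay it caches the owning BP_PlayerCharacter and registers its body, face, hair, headgear, shoulder pad, belt, glove and shoe mesh components in a map keyed by slot enum.
; ChangeDress looks up the slot's component and sets a new skeletal mesh, reinitializing its pose.
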(event `self.ReceiveBeginPlay`
  (bind _asbp_player_character (cast `/Game/MMORPG/Buleprint/Characters/BP_PlayerCharacter` (`self.GetOwner`)))
  (set `self.PlayerCharacter` _asbp_player_character)
  (`self.initDress`))

(fn `ChangeDress`
  (params (DressType :type "/Game/MMORPG/Buleprint/Characters/Player/EDress Enum" :default "NewEnumerator0") (SK :type "SkeletalMesh Object Reference"))
  (`SkinnedMeshComponent.SetSkinnedAssetAndUpdate` (`self.GetDressSlot` DressType) SK true)
  (return))

(fn `GetDressSlot`
  (params (Key :type "/Game/MMORPG/Buleprint/Characters/Player/EDress Enum" :default "NewEnumerator0"))
  (returns (Value :type "SkeletalMeshComponent Object Reference"))
  (return (`BlueprintMapLibrary.Map_Find` (`self.DressMesh`) Key)))

(fn `initDress`
  (bind _asbp_player_character (cast `/Game/MMORPG/Buleprint/Characters/BP_PlayerCharacter` (`self.GetOwner`)))
  (`self.SetDressSlot` "NewEnumerator2" (`Character.Mesh` _asbp_player_character))
  (`self.SetDressSlot` "NewEnumerator3" (`/Game/MMORPG/Buleprint/Characters/BP_PlayerCharacter.Face` _asbp_player_character))
  (`self.SetDressSlot` "NewEnumerator1" (`/Game/MMORPG/Buleprint/Characters/BP_PlayerCharacter.Belt` _asbp_player_character))
  (`self.SetDressSlot` "NewEnumerator4" (`/Game/MMORPG/Buleprint/Characters/BP_PlayerCharacter.Glove` _asbp_player_character))
  (`self.SetDressSlot` "NewEnumerator8" (`/Game/MMORPG/Buleprint/Characters/BP_PlayerCharacter.Shoe` _asbp_player_character))
  (`self.SetDressSlot` "NewEnumerator6" (`/Game/MMORPG/Buleprint/Characters/BP_PlayerCharacter.HeadGears` _asbp_player_character))
  (`self.SetDressSlot` "NewEnumerator9" (`/Game/MMORPG/Buleprint/Characters/BP_PlayerCharacter.ShoulderPad` _asbp_player_character))
  (`self.SetDressSlot` "NewEnumerator5" (`/Game/MMORPG/Buleprint/Characters/BP_PlayerCharacter.Hair` _asbp_player_character)))

(fn `SetDressSlot`
  (params (Key :type "/Game/MMORPG/Buleprint/Characters/Player/EDress Enum" :default "NewEnumerator0") (SM :type "SkeletalMeshComponent Object Reference (by ref)"))
  (`BlueprintMapLibrary.Map_Add` (`self.DressMesh`) Key SM)
  (return))
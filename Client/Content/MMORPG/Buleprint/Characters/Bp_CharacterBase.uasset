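; Base character Blueprint for the MMORPG, tying state, combat and inspectable components to overhead widgets and a trade interface.
; Cursor hover toggles inspection of the object-named character, while the info bar turns toward the camera every tick.
; Combat changes play weapon-specific equip montages, and death drops a Bp_Weapon before destroying the actor after a delay.
; Transactions open a trade widget, though closing and fulfilling are empty, and scene removal only hides the actor.
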(event `self.ReceiveBeginPlay`
  (`parent.ReceiveBeginPlay`)
  (`|ExecutionSequence`
    (:`then_0`
      (bind _asw_health_bar (cast `/Game/MMORPG/Buleprint/Characters/State/W_HealthBar` (`WidgetComponent.GetUserWidgetObject` (`self.w_HealthBar`))))
      (set `/Game/MMORPG/Buleprint/Characters/State/W_HealthBar.Entity` self _asw_health_bar))))

(event `/Game/MMORPG/Core/Common/BpI_Entity.RemoveFromScene`
  (`self.SetActorHiddenInGame` true))

(event `/Game/MMORPG/Core/Common/BpI_Entity.ReturnToScene`
  (`self.SetActorHiddenInGame` false))

(event `self.Mesh.OnBeginCursorOver`
  (params (TouchedComponent :type "PrimitiveComponent Object Reference"))
  (`/Game/MMORPG/Common/Inspect/Bpc_Inspectable.Inspect` (`self.Bpc_Inspectable`)))

(event `self.Mesh.OnEndCursorOver`
  (params (TouchedComponent :type "PrimitiveComponent Object Reference"))
  (`/Game/MMORPG/Common/Inspect/Bpc_Inspectable.UnInspect` (`self.Bpc_Inspectable`)))

(event `self.Bpc_State.OnDead`
  (`KismetSystemLibrary.Delay` 2.0)
  (`self.Drop`)
  (`self.K2_DestroyActor`))

(event `self.Bpc_Combat.OnStatuChange`
  (params (`isCombat?` :type Boolean))
  (bind _mesh (`self.Mesh`))
  (if `isCombat?`
    (`|PlayMontage` _mesh (select `/Game/MMORPG/Buleprint/Items/Weapons/EWeapon` (`/Game/MMORPG/Buleprint/Characters/Bpc_Combat.WeaponType` (`self.Bpc_Combat`)) :`NewEnumerator5` "/Game/MMORPG/Buleprint/Characters/Common/Animations/EquipmentChange_noWeaponAnim_Montage.EquipmentChange_noWeaponAnim_Montage" :`NewEnumerator0` "/Game/MMORPG/Buleprint/Characters/Common/Animations/EquipmentChange_BowAnim_Montage.EquipmentChange_BowAnim_Montage" :`NewEnumerator1` "/Game/MMORPG/Buleprint/Characters/Common/Animations/EquipmentChange_DoubleSwordAnim_Montage.EquipmentChange_DoubleSwordAnim_Montage" :`NewEnumerator2` "/Game/MMORPG/Buleprint/Characters/Common/Animations/EquipmentChange_SwordShieldAnim_Montage.EquipmentChange_SwordShieldAnim_Montage" :`NewEnumerator3` "/Game/MMORPG/Buleprint/Characters/Common/Animations/EquipmentChange01_SingleTwohandSwordAnim_Montage.EquipmentChange01_SingleTwohandSwordAnim_Montage" :`NewEnumerator4` "/Game/MMORPG/Buleprint/Characters/Common/Animations/EquipmentChange_MagicWandAnim_Montage.EquipmentChange_MagicWandAnim_Montage" :`NewEnumerator6` "/Game/MMORPG/Buleprint/Characters/Common/Animations/EquipmentChange_DoubleSwordAnim_Montage.EquipmentChange_DoubleSwordAnim_Montage" :!type "AnimMontage Object Reference"))
    (else
      (`|PlayMontage` _mesh "/Game/MMORPG/Buleprint/Characters/Common/Animations/EquipmentChange_noWeaponAnim_Montage.EquipmentChange_noWeaponAnim_Montage"))))

(event `self.ReceiveTick`
  (params (DeltaSeconds :type "Float (single-precision)"))
  (bind _returnvalue (`GameplayStatics.GetPlayerCameraManager` 0))
  (bind _w_infobar (`self.W_InfoBar`))
  ;[1 1 1] 设置头顶版时刻面向摄像机
  (`/Engine/EditorBlueprintResources/StandardMacros.IsValid` _w_infobar
    (:`Is Valid`
      (`/Engine/EditorBlueprintResources/StandardMacros.IsValid` _returnvalue
        (:`Is Valid`
          (`SceneComponent.K2_SetWorldRotation` _w_infobar (`KismetMathLibrary.FindLookAtRotation` (`SceneComponent.K2_GetComponentLocation` _w_infobar) (`self.K2_GetActorLocation` _returnvalue)) false false))))))

(event `OnTransaction`
  (bind _returnvalue (`|CreateWidget` "/Game/MMORPG/Market/W_Transaction.W_Transaction_C" (`GameplayStatics.GetPlayerController` 0) self))
  (`UserWidget.AddToViewport` _returnvalue 0))

(event `CloseTransaction`)

(event `FulfillTransaction`)

(fn `Drop`
  (returns (ReturnValue :type "/Game/MMORPG/Buleprint/Items/Weapons/Bp_Weapon Object Reference"))
  (bind _returnvalue (`|SpawnActorFromClass` "/Game/MMORPG/Buleprint/Items/Weapons/Bp_Weapon.Bp_Weapon_C" (`self.GetTransform`) "Undefined" "OverrideRootScale" null "Sword02" null))
  (return _returnvalue))

(fn `UserConstructionScript`
  (set `/Game/MMORPG/Common/Inspect/Bpc_Inspectable.name` (`KismetTextLibrary.Conv_StringToText` (`KismetSystemLibrary.GetObjectName` self)) (`self.Bpc_Inspectable`)))
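; Pre-game account pawn that handles login, registration and avatar listing, creation, deletion and world entry.
; Server request events check GameState account and avatar maps, comparing plain passwords, cache the account's avatars in PlayerState and save through the game mode.
; Client callbacks switch between login, selection and creation widgets, entering the game automatically after a successful creation.
; Entering hands the avatar and controller to the game mode's EnterWorld, then destroys this actor.
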(event `Req_Login`
  (params (Account :type String) (Password :type String))
  ;[1 1 1] 登录
  (bind _asbp_game_state (cast `/Game/MMORPG/Core/GameMode/BP_GameState` (`GameplayStatics.GetGameState`)))
  (bind (_value _returnvalue) (`BlueprintMapLibrary.Map_Find` (`/Game/MMORPG/Core/GameMode/BP_GameState.Accounts` _asbp_game_state) Account))
  (if _returnvalue
    (bind (_name _account _password) (break `/Game/MMORPG/Buleprint/Characters/Account/SAccount` _value))
    (if (`KismetStringLibrary.EqualEqual_StrStr` Password _password)
      (set `self.AccountID` _name)
      (`self.Onlogin`)
      (else
        (`KismetSystemLibrary.PrintString` "密码不对")))
    (else
      (`KismetSystemLibrary.PrintString` "没有此账号"))))

(event `Req_Register`
  (params (Account :type String) (Password :type String))
  ;[1 1 1] 注册
  (bind _asbp_game_state (cast `/Game/MMORPG/Core/GameMode/BP_GameState` (`GameplayStatics.GetGameState`)))
  (bind _accounts (`/Game/MMORPG/Core/GameMode/BP_GameState.Accounts` _asbp_game_state))
  (if (`.ReturnValue` (`BlueprintMapLibrary.Map_Find` _accounts Account))
    (`KismetSystemLibrary.PrintString` "账户已经被注册！！")
    (else
      (`BlueprintMapLibrary.Map_Add` _accounts Account (make `/Game/MMORPG/Buleprint/Characters/Account/SAccount` (`KismetStringLibrary.Conv_StringToName` Account) Account Password))
      (bind _asbp_main_game_mode (cast `/Game/MMORPG/Core/GameMode/Bp_MainGameMode` (`GameplayStatics.GetGameMode`)))
      (`/Game/MMORPG/Core/GameMode/Bp_MainGameMode.SaveGame` _asbp_main_game_mode)
      (set `self.AccountID` (`KismetStringLibrary.Conv_StringToName` Account))
      (`self.Onlogin`))))

(event `Req_AvatarList`
  (bind _asbp_player_state (cast `/Game/MMORPG/Core/Controller/Bp_PlayerState` (`self.PlayerState`)))
  (bind _asbp_game_state (cast `/Game/MMORPG/Core/GameMode/BP_GameState` (`GameplayStatics.GetGameState`)))
  (bind _values (`BlueprintMapLibrary.Map_Values` (`/Game/MMORPG/Core/GameMode/BP_GameState.Avatars` _asbp_game_state)))
  (for _array_element _values
    (bind (_name _race _transform _account) (break `/Game/MMORPG/Core/Characters/Avatar/SAvatar` _array_element))
    (if (== _account (`self.AccountID`))
      (bind _avatars (`/Game/MMORPG/Core/Controller/Bp_PlayerState.Avatars` _asbp_player_state))
      (`BlueprintMapLibrary.Map_Add` _avatars (`KismetStringLibrary.Conv_NameToString` _name) _array_element)))
  (bind _values_2 (`BlueprintMapLibrary.Map_Values` _avatars))
  (`self.OnAvatarList` _values_2))

(event `Req_CreateAvatar`
  (params (name :type String) (race :type Integer))
  (bind _returnvalue (`|GetDataTableRow` "/Game/MMORPG/Core/Characters/Race/DT_Race.DT_Race" (`KismetStringLibrary.Conv_StringToName` (`KismetStringLibrary.Conv_IntToString` race)))
    (:`then`
      (bind _asbp_game_state (cast `/Game/MMORPG/Core/GameMode/BP_GameState` (`GameplayStatics.GetGameState`)))
      ;[1 1 1] 重名检测
      (bind _keys (`BlueprintMapLibrary.Map_Keys` (`/Game/MMORPG/Core/GameMode/BP_GameState.Avatars` _asbp_game_state)))
      (for _array_element _keys
        (bind _returnvalue_2 (`KismetStringLibrary.EqualEqual_StrStr` _array_element name))
        (if _returnvalue_2
          (break)))
      (if (not _returnvalue_2)
        (bind _asbp_main_game_mode (cast `/Game/MMORPG/Core/GameMode/Bp_MainGameMode` (`GameplayStatics.GetGameMode`)))
        (bind ((`race_55_B3C67C9B4586507DC86CC4B8A0A8153E` _race) (`Position_54_A10CEAFB41012EC7B6EEC8B10DCCBE62` _position)) (break `/Game/MMORPG/Core/Characters/Race/SRace` _returnvalue))
        (bind _savatar (make `/Game/MMORPG/Core/Characters/Avatar/SAvatar` (`KismetStringLibrary.Conv_StringToName` name) _race _position (`self.AccountID`)))
        (`/Game/MMORPG/Core/GameMode/Bp_MainGameMode.CreateAvatar` _asbp_main_game_mode _savatar)
        (bind _asbp_player_state (cast `/Game/MMORPG/Core/Controller/Bp_PlayerState` (`self.PlayerState`)))
        (`BlueprintMapLibrary.Map_Add` (`/Game/MMORPG/Core/Controller/Bp_PlayerState.Avatars` _asbp_player_state) name _savatar)
        (`self.OnCreateAvatar` _savatar true)
        (else
          (`self.OnCreateAvatar` (make `/Game/MMORPG/Core/Characters/Avatar/SAvatar`)))))))

(event `Req_EnterGame`
  (params (Avatar :type String))
  (bind _asbp_main_game_mode (cast `/Game/MMORPG/Core/GameMode/Bp_MainGameMode` (`GameplayStatics.GetGameMode`)))
  (bind _asbp_player_controller (cast `/Game/MMORPG/Core/Controller/Bp_PlayerController` (`self.GetController`)))
  (bind _asbp_player_state (cast `/Game/MMORPG/Core/Controller/Bp_PlayerState` (`self.PlayerState`)))
  (`/Game/MMORPG/Core/GameMode/Bp_MainGameMode.EnterWorld` _asbp_main_game_mode (`BlueprintMapLibrary.Map_Find` (`/Game/MMORPG/Core/Controller/Bp_PlayerState.Avatars` _asbp_player_state) Avatar) _asbp_player_controller)
  (`self.K2_DestroyActor`))

(event `Req_DelAvatar`
  (params (AvatarName :type String))
  (bind _asbp_game_state (cast `/Game/MMORPG/Core/GameMode/BP_GameState` (`GameplayStatics.GetGameState`)))
  (`BlueprintMapLibrary.Map_Remove` (`/Game/MMORPG/Core/GameMode/BP_GameState.Avatars` _asbp_game_state) AvatarName)
  (bind _asbp_player_state (cast `/Game/MMORPG/Core/Controller/Bp_PlayerState` (`self.PlayerState`)))
  (bind _avatars (`/Game/MMORPG/Core/Controller/Bp_PlayerState.Avatars` _asbp_player_state))
  (`BlueprintMapLibrary.Map_Remove` _avatars AvatarName)
  (bind _asbp_main_game_mode (cast `/Game/MMORPG/Core/GameMode/Bp_MainGameMode` (`GameplayStatics.GetGameMode`)))
  (`/Game/MMORPG/Core/GameMode/Bp_MainGameMode.SaveGame` _asbp_main_game_mode)
  (bind _values (`BlueprintMapLibrary.Map_Values` _avatars))
  (`self.OnDelAvatar` _values))

(event `OnLogin`
  (`Widget.RemoveFromParent` (`self.W_LoginMain`))
  (`self.Req_AvatarList`))

(event `OnAvatarList`
  (params (Avatars :type "Array of /Game/MMORPG/Core/Characters/Avatar/SAvatar Structure"))
  (set `self.AvatarList` Avatars)
  (if (not (<= (`KismetArrayLibrary.Array_Length` Avatars) 0))
    (bind _returnvalue (`|CreateWidget` "/Game/MMORPG/Maps/SelectAvatar/W_SelectAvatar.W_SelectAvatar_C"))
    (bind _output_get (set `self.W_SelecteAvatar` _returnvalue))
    (`UserWidget.AddToViewport` _output_get 0)
    (else
      (bind _returnvalue_2 (`|CreateWidget` "/Game/MMORPG/Maps/SelectAvatar/W_CreateAvatar.W_CreateAvatar_C"))
      (bind _output_get_2 (set `self.W_CreateAvatar` _returnvalue_2))
      (`UserWidget.AddToViewport` _output_get_2 0))))

(event `OnDelAvatar`
  (params (AvatarList :type "Array of /Game/MMORPG/Core/Characters/Avatar/SAvatar Structure"))
  (set `self.AvatarList` AvatarList)
  (`/Game/MMORPG/Maps/SelectAvatar/W_SelectAvatar.UpdateAvatarList` (`self.W_SelecteAvatar`)))

(event `OnCreateAvatar`
  (params (Avatar :type "/Game/MMORPG/Core/Characters/Avatar/SAvatar Structure") (canCreate :type Boolean))
  (bind _returnvalue (`KismetStringLibrary.Conv_NameToString` (`.Name_12_29693B144F53C8E3D43900A0D1079529` (break `/Game/MMORPG/Core/Characters/Avatar/SAvatar` Avatar))))
  (if canCreate
    (`KismetSystemLibrary.PrintString` "创建成功！")
    (`Widget.RemoveFromParent` (`self.W_CreateAvatar`))
    (`self.Req_EnterGame` _returnvalue)
    (else
      (`KismetSystemLibrary.PrintString` (`KismetStringLibrary.Concat_StrStr` _returnvalue "——名字重复，无法创建！")))))

(fn `UserConstructionScript`)
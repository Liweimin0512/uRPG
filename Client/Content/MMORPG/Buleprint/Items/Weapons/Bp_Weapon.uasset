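; Weapon item Blueprint that configures itself from equipment and weapon data tables and carries a BpCWeapon component.
; After the parent construction script, it looks up EquipID in DT_Equip to resolve WeaponID, falling back to EquipID when that is None.
; The DT_Weapon row then sets the component's weapon type and the name, using the equipment name if the weapon's is empty.
; BeginPlay clears the component's owner character.
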(event `self.ReceiveBeginPlay`
  (set `/Game/MMORPG/Buleprint/Items/Bpc_Weapon.ownerCharacter` null (`self.BpC_Weapon`)))

(fn `UserConstructionScript`
  (locals (LocalEquipName :type Text))
  (`parent.UserConstructionScript`)
  (bind _returnvalue (`|GetDataTableRow` "/Game/MMORPG/Buleprint/Items/Equip/DT_Equip.DT_Equip" (`self.EquipID`))
    (:`then`
      (bind (_name _slot _weaponid) (break `/Game/MMORPG/Buleprint/Items/Equip/SEquip` _returnvalue))
      (set `local.LocalEquipName` _name)
      (bind _output_get (set `self.WeaponID` (select `bool` (!= _weaponid "None") :`false` (`self.EquipID`) :`true` _weaponid)))
      (bind _returnvalue_2 (`|GetDataTableRow` "/Game/MMORPG/Buleprint/Items/Weapons/DT_Weapon.DT_Weapon" _output_get)
        (:`then`
          (bind (_name_2 _meshpic _weapontype) (break `/Game/MMORPG/Buleprint/Items/Weapons/s_Weapon` _returnvalue_2))
          (set `self.Name` (select `bool` (`KismetTextLibrary.TextIsEmpty` _name_2) :`false` _name_2 :`true` (`local.LocalEquipName`)))
          (set `/Game/MMORPG/Buleprint/Items/Bpc_Weapon.WeaponType` _weapontype (`self.BpC_Weapon`)))))))
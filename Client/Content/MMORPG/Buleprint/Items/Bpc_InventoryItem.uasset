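; Actor component that makes its owning item actor an inventory item that characters can hold and drop.
; Storing records the owning character, attaches the item to it and messages it to leave the scene; dropping detaches, unhides and moves it to a location.
; Put-in and drop events call out to callback functions.
; Helpers expose the owner's BpcInventory and a distance-based pickup check, while slot lookup and RemoveFromOwner are unfinished.
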(event `OnPutInInventory`
  (params (ownerCha :type "/Game/MMORPG/Buleprint/Characters/Bp_CharacterBase Object Reference"))
  (bind _returnvalue (`self.GetOwner`))
  (`self.SetOwner` ownerCha)
  (`Actor.K2_AttachToActor` _returnvalue (`self.ownerCharacter`) "None" "SnapToTarget" "SnapToTarget" "SnapToTarget" true)
  (message `/Game/MMORPG/Core/Common/BpI_Entity.RemoveFromScene` _returnvalue)
  (`self.OnPutinInventoryFn` (`self.ownerCharacter`)))

(event `OnRemoved`
  (bind _returnvalue (`self.GetOwner`))
  (`/Engine/EditorBlueprintResources/StandardMacros.IsValid` (`self.ownerCharacter`)
    (:`Is Valid`
      (`Actor.K2_DetachFromActor` _returnvalue "KeepRelative" "KeepRelative" "KeepRelative")
      (`self.ClearOwner`)
      (`Actor.SetActorHiddenInGame` _returnvalue false))))

(event `OnDropped`
  (bind _returnvalue (`self.GetOwner`))
  (bind _ownercharacter (`self.ownerCharacter`))
  (`/Engine/EditorBlueprintResources/StandardMacros.IsValid` _returnvalue
    (:`Is Valid`
      (`self.OnRemoved`)
      (`Actor.K2_SetActorLocation` (`self.GetOwner`) (select `bool` (`KismetSystemLibrary.IsValid` _ownercharacter) :`false` (`Actor.K2_GetActorLocation` _returnvalue) :`true` (`Actor.K2_GetActorLocation` _ownercharacter)) false false)
      (`self.OnDropFn`))))

(fn `canPickup`
  (params (targetCharacter :type "/Game/MMORPG/Buleprint/Characters/Bp_CharacterBase Object Reference"))
  (returns (ReturnValue :type Boolean))
  (bind _returnvalue (`KismetMathLibrary.VSize` (- (`Actor.K2_GetActorLocation` (`self.GetOwner`)) (`Actor.K2_GetActorLocation` targetCharacter))))
  (`KismetSystemLibrary.PrintString` (`KismetStringLibrary.Conv_DoubleToString` _returnvalue))
  (return (<= _returnvalue 300.0)))

(fn `ClearOwner`
  (set `self.ownerCharacter` null)
  (return))

(fn `GetContainer`
  (returns (Bpc_Inventory :type "/Game/MMORPG/Buleprint/Characters/Inventory/BPC_Inventory Object Reference"))
  (bind _ownercharacter (`self.ownerCharacter`))
  (`/Engine/EditorBlueprintResources/StandardMacros.IsValid` _ownercharacter
    (:`Is Valid`
      (return (`/Game/MMORPG/Buleprint/Characters/Bp_CharacterBase.Bpc_Inventory` _ownercharacter)))))

(fn `GetDebugString`
  (returns (Image :type Text))
  (return (`|FormatText` "inventory image name set to:{imagename}" (`KismetTextLibrary.Conv_NameToText` (`self.imageName`)))))

(fn `GetSlotNum`
  (locals (ct :type "/Game/MMORPG/Buleprint/Characters/Inventory/BPC_Inventory Object Reference"))
  (bind _ownercharacter (`self.ownerCharacter`))
  (`/Engine/EditorBlueprintResources/StandardMacros.IsValid` _ownercharacter
    (:`Is Valid`
      (bind _output_get (set `local.ct` (`/Game/MMORPG/Buleprint/Characters/Bp_CharacterBase.Bpc_Inventory` _ownercharacter)))
      (`/Engine/EditorBlueprintResources/StandardMacros.IsValid` _output_get
        (:`Is Valid`
          (return))))))

(fn `RemoveFromOwner`)

(fn `SetOnActiveItemFn`
  (params (fn :type Name))
  (set `self.onActiveitemFn` fn)
  (return))

(fn `SetOnDroppedFn`
  (params (fn :type Name)))

(fn `SetOwner`
  (params (ownerCha :type "/Game/MMORPG/Buleprint/Characters/Bp_CharacterBase Object Reference"))
  (set `self.ownerCharacter` ownerCha)
  (return))
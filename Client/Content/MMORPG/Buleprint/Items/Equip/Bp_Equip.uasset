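; Bp_Equip is an equippable item actor that configures itself from data tables in its construction script.
; After running the parent script, it finds its ItemID row in DT_Item and derives the EquipID, falling back to ItemID when Equip is None.
; The matching DT_Equip row supplies EquipName, falling back to the item name if empty, and the Slot copied into BpcEquippable.
; The event graph has no active logic.
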(fn `UserConstructionScript`
  (locals (LocalItemName :type Text))
  (`parent.UserConstructionScript`)
  (bind _returnvalue (`|GetDataTableRow` "/Game/MMORPG/Buleprint/Items/DT_Item.DT_Item" (`self.ItemID`))
    (:`then`
      (bind (_name _type _stacklimit _itemicon _itemcolor _weight _use _equip) (break `/Game/MMORPG/Buleprint/Items/SItem` _returnvalue))
      (set `local.LocalItemName` _name)
      (bind _output_get (set `self.EquipID` (select `bool` (!= _equip "None") :`false` (`self.ItemID`) :`true` _equip)))
      (bind _returnvalue_2 (`|GetDataTableRow` "/Game/MMORPG/Buleprint/Items/Equip/DT_Equip.DT_Equip" _output_get)
        (:`then`
          (bind (_name_2 _slot) (break `/Game/MMORPG/Buleprint/Items/Equip/SEquip` _returnvalue_2))
          (set `self.equipName` (select `bool` (`KismetTextLibrary.TextIsEmpty` _name_2) :`false` _name_2 :`true` (`local.LocalItemName`)))
          (bind _output_get_2 (set `self.Slot` _slot))
          (set `/Game/MMORPG/Buleprint/Items/Bpc_Equippable.EquipSolt` _output_get_2 (`self.Bpc_Equippable`)))))))
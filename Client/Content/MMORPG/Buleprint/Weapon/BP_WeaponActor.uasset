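; BP_WeaponActor is a melee weapon actor that detects hits through a capsule whose collision is enabled only during attack windows.
; Overlapping an actor of a different class from the instigator sends the stored attack event tag to the instigator as a gameplay event, targeting that actor.
; A DoOnce gate, reset shortly after overlap ends, limits repeat hits.
; Hits can trigger a count-limited hit pause through brief global time dilation, using fixed delays rather than the stored delay time.
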(event `self.ReceiveBeginPlay`
  (`PrimitiveComponent.IgnoreActorWhenMoving` (`self.Capsule`) null false))

(event `Event BeginWeaponAttack`
  (params (EventTag :type "GameplayTag Structure") (AttackDelayTime :type "Float (double-precision)") (AttackDelayCount :type Integer))
  (set `self.AttackEventTag` EventTag)
  (set `self.AttackDelayTime` AttackDelayTime)
  (set `self.AttackDelayCount` AttackDelayCount)
  (set `self.IsAttacking` true)
  (`PrimitiveComponent.SetCollisionEnabled` (`self.Capsule`) "QueryOnly"))

(event `Event EndWeaponAttack`
  (set `self.IsAttacking` false)
  (`PrimitiveComponent.SetCollisionEnabled` (`self.Capsule`) "NoCollision"))

(event `self.ReceiveActorBeginOverlap`
  (params (OtherActor :type "Actor Object Reference"))
  (bind _returnvalue (`self.GetInstigator`))
  (if (and (!= (`GameplayStatics.GetObjectClass` OtherActor) (`GameplayStatics.GetObjectClass` (`self.GetInstigator`))) (`self.IsAttacking`))
    (`/Engine/EditorBlueprintResources/StandardMacros.DoOnce` false :!label _label
      (:`Completed`
        (`AbilitySystemBlueprintLibrary.SendGameplayEventToActor` _returnvalue (`self.AttackEventTag`) (make `GameplayEventData` (struct) _returnvalue OtherActor))
        (`self.HitPause`)))))

(event `self.ReceiveActorEndOverlap`
  (params (OtherActor :type "Actor Object Reference"))
  (`KismetSystemLibrary.Delay` 0.2)
  (goto _label :!via `Reset`))

(event `HitPause`
  (if (and (> (`self.AttackDelayCount`) 0) (`self.EnableAttackDelay`))
    (`/Engine/EditorBlueprintResources/StandardMacros.DecrementInt` (`self.AttackDelayCount`)
      (:`  `
        (`KismetSystemLibrary.Delay` 0.1)
        (`GameplayStatics.SetGlobalTimeDilation` 0.1)
        (`KismetSystemLibrary.Delay` 0.01)
        (`GameplayStatics.SetGlobalTimeDilation` 1.0)))))

(fn `UserConstructionScript`)
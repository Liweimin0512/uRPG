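; Weapon component for MMORPG item actors that attaches the weapon to its wielder and delivers melee hits.
; On Bpc_Equippable's OnEquip it stores the owner and snaps to the right-hand weapon socket for every weapon type.
; Actor overlaps call OnHit on the other actor's Bpc_Combat while the wielder's combat flags are set.
; It also holds damage, range and projectile settings, with stubbed ranged checks and projectile spawning at world origin.
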(event `OnEquip_事件_0`
  (params (ownerCharacter :type "/Game/MMORPG/Core/Characters/Bp_CharacterBase Object Reference"))
  (bind _output_get (set `self.ownerCharacter` ownerCharacter))
  (`Actor.K2_AttachToActor` (`self.GetOwner`) _output_get (select `/Game/MMORPG/Items/Weapons/EWeapon` (`self.WeaponType`) :`NewEnumerator5` "Socket_WeaponPositionRight" :`NewEnumerator0` "Socket_WeaponPositionRight" :`NewEnumerator1` "Socket_WeaponPositionRight" :`NewEnumerator2` "Socket_WeaponPositionRight" :`NewEnumerator3` "Socket_WeaponPositionRight" :`NewEnumerator4` "Socket_WeaponPositionRight" :`NewEnumerator6` "Socket_WeaponPositionRight" :!type "Name") "SnapToTarget" "SnapToTarget" "SnapToTarget" false))

(event `self.ReceiveBeginPlay`
  (bind _returnvalue (`self.GetOwner`))
  (bind _returnvalue_2 (`Actor.GetComponentByClass` (`self.GetOwner`) "/Game/MMORPG/Core/Item/Bpc_Equippable.Bpc_Equippable_C"))
  (`|ExecutionSequence`
    (:`then_0`
      (`/Engine/EditorBlueprintResources/StandardMacros.IsValid` _returnvalue_2
        (:`Is Valid`
          (add `/Game/MMORPG/Core/Item/Bpc_Equippable.OnEquip` _returnvalue_2 (delegate `OnEquip_事件_0`)))))
    (:`then_2`
      (`/Engine/EditorBlueprintResources/StandardMacros.IsValid` _returnvalue
        (:`Is Valid`
          (add `Actor.OnActorBeginOverlap` _returnvalue (delegate `OnActorBeginOverlap_事件_0`)))))))

(event `OnActorBeginOverlap_事件_0`
  (params (OverlappedActor :type "Actor Object Reference") (OtherActor :type "Actor Object Reference"))
  (bind _returnvalue (`Actor.GetComponentByClass` OtherActor "/Game/MMORPG/Core/Characters/Bpc_Combat.Bpc_Combat_C"))
  (bind _ownercharacter (`self.ownerCharacter`))
  (`/Engine/EditorBlueprintResources/StandardMacros.IsValid` _ownercharacter
    (:`Is Valid`
      (if (and (!= OtherActor _ownercharacter) (`/Game/MMORPG/Core/Characters/Bpc_Combat.isHit?` (`Actor.GetComponentByClass` _ownercharacter "/Game/MMORPG/Core/Characters/Bpc_Combat.Bpc_Combat_C")))
        (if (`/Game/MMORPG/Core/Characters/Bpc_Combat.isAttack?` (`Actor.GetComponentByClass` _ownercharacter "/Game/MMORPG/Core/Characters/Bpc_Combat.Bpc_Combat_C"))
          (`/Engine/EditorBlueprintResources/StandardMacros.IsValid` _returnvalue
            (:`Is Valid`
              (`/Game/MMORPG/Core/Characters/Bpc_Combat.OnHit` _returnvalue null (`self.GetOwner`)))
            (:`Is Not Valid`
              (`KismetSystemLibrary.PrintString` "hiter has no combat component"))))
        (else
          (`KismetSystemLibrary.PrintString` "is not attack"))))))

(event `self.ReceiveEndPlay`
  (params (EndPlayReason :type "EEndPlayReason Enum" :default "Destroyed"))
  (remove `Actor.OnActorBeginOverlap` (`self.GetOwner`) (delegate `OnActorBeginOverlap_事件_0`)))

(fn `CanRangedAttack`
  (returns (canRangedAttack :type Boolean))
  (return true))

(fn `LaunchProjectile`
  (params (attacker :type "Actor Object Reference") (target :type "Actor Object Reference"))
  (locals (proj :type "Actor Object Reference"))
  (bind _projectile (`self.projectile`))
  (`/Engine/EditorBlueprintResources/StandardMacros.IsValid` _projectile
    (:`Is Valid`
      (`self.onprojectilelaunchfn` attacker target)
      (`|SpawnActorFromClass` (`GameplayStatics.GetObjectClass` _projectile) (`KismetMathLibrary.MakeTransform` (0.0 0.0 0.0)) "Undefined" "OverrideRootScale" null null))))

(fn `SetDamage`
  (params (damage :type Integer))
  (set `self.damage` damage)
  (return))

(fn `SetProjectile`
  (params (projectile :type "Actor Object Reference"))
  (set `self.projectile` projectile))

(fn `SetRange`
  (params (attackrange :type Integer) (hitrange :type Integer))
  (set `self.attackrange` attackrange)
  (set `self.hitrange` hitrange)
  (return))
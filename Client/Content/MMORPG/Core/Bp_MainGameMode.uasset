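; Main game mode for the MMORPG, managing accounts, avatars and entry into the game world.
; BeginPlay restores accounts and avatars from the "Account" save slot into BP_GameState and caches the level's buildings.
; New logins possess a spawned BP_Account pawn; entering the world spawns and possesses a BP_PlayerCharacter at the avatar's transform, tracked in PlayerList.
; Creating an avatar registers it by name and rewrites the save.
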(event `self.ReceiveBeginPlay`
  (`self.LoadGame`)
  (bind _outactors (`GameplayStatics.GetAllActorsOfClass` "/Game/MMORPG/Building/BP_Building.BP_Building_C"))
  (set `self.Buildings` _outactors))

(event `ClientTravel`
  (params (SpecificPlayer :type "PlayerController Object Reference") (B :type String))
  (`KismetSystemLibrary.ExecuteConsoleCommand` (`KismetStringLibrary.Concat_StrStr` "clienttravel " B) SpecificPlayer))

(event `self.K2_PostLogin`
  (params (NewPlayer :type "PlayerController Object Reference"))
  (bind _returnvalue (`|SpawnActorFromClass` "/Game/MMORPG/Core/Characters/Account/BP_Account.BP_Account_C" (`KismetMathLibrary.MakeTransform` (0.0 0.0 0.0)) "Undefined" "OverrideRootScale" null null))
  (`Controller.Possess` NewPlayer _returnvalue))

(event `CreateAvatar`
  (params (Avatar :type "/Game/MMORPG/Core/Characters/Avatar/SAvatar Structure"))
  (bind _asbp_game_state (cast `/Game/MMORPG/Core/BP_GameState` (`GameplayStatics.GetGameState`)))
  (`BlueprintMapLibrary.Map_Add` (`/Game/MMORPG/Core/BP_GameState.Avatars` _asbp_game_state) (`KismetStringLibrary.Conv_NameToString` (`.Name_12_29693B144F53C8E3D43900A0D1079529` (break `/Game/MMORPG/Core/Characters/Avatar/SAvatar` Avatar))) Avatar)
  (`self.SaveGame`))

(event `EnterWorld`
  (params (Avatar :type "/Game/MMORPG/Core/Characters/Avatar/SAvatar Structure") (controller :type "/Game/MMORPG/Core/Controller/Bp_PlayerController Object Reference"))
  (bind ((`Name_12_29693B144F53C8E3D43900A0D1079529` _name) (`Transform_7_89C660774663419BBCA4B39FE7D79D26` _transform)) (break `/Game/MMORPG/Core/Characters/Avatar/SAvatar` Avatar))
  (bind _returnvalue (`|SpawnActorFromClass` "/Game/MMORPG/Characters/Player/BP_PlayerCharacter.BP_PlayerCharacter_C" _transform "AdjustIfPossibleButAlwaysSpawn" "OverrideRootScale" null (struct) (`KismetStringLibrary.Conv_NameToString` _name) null))
  (`KismetArrayLibrary.Array_Add` (`self.PlayerList`) _returnvalue)
  (`Controller.Possess` controller _returnvalue))

(event `LeavelWorld`
  (params (Player :type "/Game/MMORPG/Characters/Player/BP_PlayerCharacter Object Reference"))
  (`KismetArrayLibrary.Array_RemoveItem` (`self.PlayerList`) Player))

(fn `LoadGame`
  (bind _returnvalue (`GameplayStatics.LoadGameFromSlot` "Account"))
  (bind _asbp_save_game (cast `/Game/MMORPG/Core/Bp_SaveGame` _returnvalue))
  (bind _asbp_game_state (cast `/Game/MMORPG/Core/BP_GameState` (`GameplayStatics.GetGameState`)))
  (set `/Game/MMORPG/Core/BP_GameState.Accounts` (`/Game/MMORPG/Core/Bp_SaveGame.Accounts` _asbp_save_game) _asbp_game_state)
  (set `/Game/MMORPG/Core/BP_GameState.Avatars` (`/Game/MMORPG/Core/Bp_SaveGame.Avatars` _asbp_save_game) _asbp_game_state))

(fn `SaveGame`
  (bind _returnvalue (`GameplayStatics.DoesSaveGameExist` "Account"))
  (if _returnvalue
    _
    (else
      _))
  (bind _returnvalue_2 (`GameplayStatics.CreateSaveGameObject` "/Game/MMORPG/Core/Bp_SaveGame.Bp_SaveGame_C"))
  (bind _asbp_game_state (cast `/Game/MMORPG/Core/BP_GameState` (`GameplayStatics.GetGameState`)))
  (set `/Game/MMORPG/Core/Bp_SaveGame.Accounts` (`/Game/MMORPG/Core/BP_GameState.Accounts` _asbp_game_state) _returnvalue_2)
  (set `/Game/MMORPG/Core/Bp_SaveGame.Avatars` (`/Game/MMORPG/Core/BP_GameState.Avatars` _asbp_game_state) _returnvalue_2)
  (`GameplayStatics.SaveGameToSlot` _returnvalue_2 "Account"))

(fn `UserConstructionScript`)
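; Player controller for the MMORPG that shows the login UI and requests map travel.
; On BeginPlay it creates the W_LoginMain widget, stores it on the BP_Account pawn and adds it to the viewport.
; Pressing Q requests client travel to Map01, apparently as a test shortcut.
; The Req_ClientTravel event forwards travel requests to Bp_MainGameMode, passing itself as the player to move.
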(event `self.ReceiveBeginPlay`
  (bind _returnvalue (`|CreateWidget` "/Game/MMORPG/Maps/LoginAndRegister/W_LoginMain.W_LoginMain_C" (`GameplayStatics.GetPlayerController` 0)))
  (bind _asbp_account (cast `/Game/MMORPG/Core/Characters/Account/BP_Account` (`GameplayStatics.GetPlayerPawn` 0)))
  (bind _output_get (set `/Game/MMORPG/Core/Characters/Account/BP_Account.W_LoginMain` _returnvalue _asbp_account))
  (`/Engine/EditorBlueprintResources/StandardMacros.IsValid` _output_get
    (:`Is Valid`
      (`UserWidget.AddToViewport` _output_get 0))))

(event `Key|Q`
  (params (Key :type "Key Structure"))
  (:`Pressed`
    (`self.Req_ClientTravel` "Map01")))

(event `Req_ClientTravel`
  (params (B :type String))
  (bind _asbp_main_game_mode (cast `/Game/MMORPG/Core/GameMode/Bp_MainGameMode` (`GameplayStatics.GetGameMode`)))
  (`/Game/MMORPG/Core/GameMode/Bp_MainGameMode.ClientTravel` _asbp_main_game_mode self B))

(fn `UserConstructionScript`)
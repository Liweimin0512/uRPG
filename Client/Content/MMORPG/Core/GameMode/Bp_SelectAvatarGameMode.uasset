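; Game mode for the MMORPG avatar selection screen, driven by KBEngine event data.
; On start it shows the cursor and stores the placed player character; the received avatar list then opens either the selection or creation widget.
; Creation and removal events update the cached list and selection UI, while a space geometry mapping event opens the level named in its resource path.
; UpdateSelectModel is an empty stub.
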(event `self.ReceiveBeginPlay`
  (set `PlayerController.bShowMouseCursor` true (`GameplayStatics.GetPlayerController` 0))
  (bind _outactors (`GameplayStatics.GetAllActorsOfClass` "/Game/MMORPG/Characters/BP_PlayerCharacter.BP_PlayerCharacter_C"))
  (set `self.Ref_Avatar` (`|GetArrayItem` _outactors)))

(event `self.onReqAvatarList`
  (params (pEventData :type "KBEventData Object Reference"))
  ;[1 1 1] 返回角色信息
  (bind _askbevent_data_on_req_avatar_list (cast `KBEventData_onReqAvatarList` pEventData))
  (bind _avatars (`KBEventData_onReqAvatarList.avatars` _askbevent_data_on_req_avatar_list))
  (set `self.Avatars` _avatars)
  (if (> (`KismetArrayLibrary.Array_Length` _avatars) 0)
    (bind _returnvalue (`|CreateWidget` "/Game/MMORPG/Maps/SelectAvatar/UMG_SelectAvatar.UMG_SelectAvatar_C"))
    (bind _output_get (set `self.Ref_selectUI` _returnvalue))
    (`UserWidget.AddToViewport` _output_get 0)
    (else
      (bind _returnvalue_2 (`|CreateWidget` "/Game/MMORPG/Maps/SelectAvatar/UMG_CreateAvatar.UMG_CreateAvatar_C"))
      (`UserWidget.AddToViewport` _returnvalue_2 0))))

(event `self.onCreateAvatarResult`
  (params (pEventData :type "KBEventData Object Reference"))
  (bind _askbevent_data_on_create_avatar_result (cast `KBEventData_onCreateAvatarResult` pEventData))
  (`KismetSystemLibrary.PrintString` (`KBEventData_onCreateAvatarResult.errorStr` _askbevent_data_on_create_avatar_result))
  (bind _avatarinfos (`KBEventData_onCreateAvatarResult.avatarInfos` _askbevent_data_on_create_avatar_result))
  (`KismetSystemLibrary.PrintString` (`KismetTextLibrary.Conv_TextToString` (`|FormatText` "创建角色完成{0}" (`KismetTextLibrary.Conv_StringToText` (`.name` (break `AVATAR_INFOS` _avatarinfos))))))
  (`KismetArrayLibrary.Array_Add` (`self.Avatars`) _avatarinfos)
  (bind _returnvalue (`|CreateWidget` "/Game/MMORPG/Maps/SelectAvatar/UMG_SelectAvatar.UMG_SelectAvatar_C"))
  (bind _output_get (set `self.Ref_selectUI` _returnvalue))
  (`UserWidget.AddToViewport` _output_get 0))

(event `self.onRemoveAvatar`
  (params (pEventData :type "KBEventData Object Reference"))
  ;[1 1 1] 当角色删除
  (bind _askbevent_data_on_remove_avatar (cast `KBEventData_onRemoveAvatar` pEventData))
  (`KismetArrayLibrary.Array_RemoveItem` (`self.Avatars`) (`KBEventData_onRemoveAvatar.avatarInfos` _askbevent_data_on_remove_avatar))
  (`/Game/MMORPG/Maps/SelectAvatar/UMG_SelectAvatar.updateAvatarList` (`self.Ref_selectUI`)))

(event `self.addSpaceGeometryMapping`
  (params (pEventData :type "KBEventData Object Reference"))
  (bind _askbevent_data_add_space_geometry_mapping (cast `KBEventData_addSpaceGeometryMapping` pEventData))
  (bind (_lefts _rights) (`KismetStringLibrary.Split` (`KBEventData_addSpaceGeometryMapping.spaceResPath` _askbevent_data_add_space_geometry_mapping) "/"))
  (`GameplayStatics.OpenLevel` (`KismetStringLibrary.Conv_StringToName` _rights))
  (`KismetSystemLibrary.PrintString` _rights))

(fn `updateSelectModel`
  (params (chapic :type "/Game/MMORPG/Core/s_RacePic Structure")))

(fn `UserConstructionScript`)
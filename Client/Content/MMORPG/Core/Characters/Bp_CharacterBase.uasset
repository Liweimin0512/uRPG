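; Base character Blueprint for the MMORPG, registering itself by EntityID with Bp_MainGameMode on BeginPlay and binding to its health bar widget.
; Cursor hover toggles the inspectable component, named after the object, and combat status changes play equipment-change montages chosen by weapon type.
; On death it waits, spawns a Bp_Weapon drop and destroys itself, though Destroyed removes entity 0 instead of its own EntityID.
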(event `self.ReceiveBeginPlay`
  (`parent.ReceiveBeginPlay`)
  (`|ExecutionSequence`
    (:`then_0`
      (bind _output_get (set `self.GameMode` (cast `/Game/MMORPG/Core/GameMode/Bp_MainGameMode` (`GameplayStatics.GetGameMode`) :!pure true)))
      (`/Engine/EditorBlueprintResources/StandardMacros.IsValid` _output_get
        (:`Is Valid`
          (`/Game/MMORPG/Core/GameMode/Bp_MainGameMode.addGameEntity` (`self.GameMode`) (`self.entityID`) self))))
    (:`then_1`
      (bind _asw_health_bar (cast `/Game/MMORPG/Characters/Common/w_HealthBar` (`WidgetComponent.GetUserWidgetObject` (`self.w_HealthBar`))))
      (set `/Game/MMORPG/Characters/Common/w_HealthBar.Entity` self _asw_health_bar))))

(event `self.ReceiveDestroyed`
  (bind _gamemode (`self.GameMode`))
  (`parent.ReceiveDestroyed`)
  (`/Engine/EditorBlueprintResources/StandardMacros.IsValid` _gamemode
    (:`Is Valid`
      (`/Game/MMORPG/Core/GameMode/Bp_MainGameMode.removeGameEntity` _gamemode 0))))

(event `self.collect_collision.OnComponentBeginOverlap`
  (params (OverlappedComponent :type "PrimitiveComponent Object Reference") (OtherActor :type "Actor Object Reference") (OtherComp :type "PrimitiveComponent Object Reference") (OtherBodyIndex :type Integer) (bFromSweep :type Boolean) (SweepResult :type "HitResult Structure (by ref)"))
  (if (!= OtherActor self)
    (`KismetSystemLibrary.PrintString` (`KismetSystemLibrary.GetObjectName` OtherActor))))

(event `self.Mesh.OnBeginCursorOver`
  (params (TouchedComponent :type "PrimitiveComponent Object Reference"))
  (`/Game/MMORPG/Inspect/Bpc_Inspectable.Inspect` (`self.Bpc_Inspectable`)))

(event `self.Mesh.OnEndCursorOver`
  (params (TouchedComponent :type "PrimitiveComponent Object Reference"))
  (`/Game/MMORPG/Inspect/Bpc_Inspectable.UnInspect` (`self.Bpc_Inspectable`)))

(event `self.Bpc_State.OnDead`
  (`KismetSystemLibrary.Delay` 2.0)
  (`self.Drop`)
  (`self.K2_DestroyActor`))

(event `self.Bpc_Combat.OnStatuChange`
  (params (`isCombat?` :type Boolean))
  (bind _mesh (`self.Mesh`))
  (if `isCombat?`
    (`|PlayMontage` _mesh (select `/Game/MMORPG/Items/Weapons/EWeapon` (`/Game/MMORPG/Core/Characters/Bpc_Combat.WeaponType` (`self.Bpc_Combat`)) :`NewEnumerator5` "/Game/MMORPG/Characters/Common/Animations/EquipmentChange_noWeaponAnim_Montage.EquipmentChange_noWeaponAnim_Montage" :`NewEnumerator0` "/Game/MMORPG/Characters/Common/Animations/EquipmentChange_BowAnim_Montage.EquipmentChange_BowAnim_Montage" :`NewEnumerator1` "/Game/MMORPG/Characters/Common/Animations/EquipmentChange_DoubleSwordAnim_Montage.EquipmentChange_DoubleSwordAnim_Montage" :`NewEnumerator2` "/Game/MMORPG/Characters/Common/Animations/EquipmentChange_SwordShieldAnim_Montage.EquipmentChange_SwordShieldAnim_Montage" :`NewEnumerator3` "/Game/MMORPG/Characters/Common/Animations/EquipmentChange01_SingleTwohandSwordAnim_Montage.EquipmentChange01_SingleTwohandSwordAnim_Montage" :`NewEnumerator4` "/Game/MMORPG/Characters/Common/Animations/EquipmentChange_MagicWandAnim_Montage.EquipmentChange_MagicWandAnim_Montage" :`NewEnumerator6` "/Game/MMORPG/Characters/Common/Animations/EquipmentChange_DoubleSwordAnim_Montage.EquipmentChange_DoubleSwordAnim_Montage" :!type "AnimMontage Object Reference"))
    (else
      (`|PlayMontage` _mesh "/Game/MMORPG/Characters/Common/Animations/EquipmentChange_noWeaponAnim_Montage.EquipmentChange_noWeaponAnim_Montage"))))

(event `self.Box.OnComponentBeginOverlap`
  (params (OverlappedComponent :type "PrimitiveComponent Object Reference") (OtherActor :type "Actor Object Reference") (OtherComp :type "PrimitiveComponent Object Reference") (OtherBodyIndex :type Integer) (bFromSweep :type Boolean) (SweepResult :type "HitResult Structure (by ref)"))
  (if (!= OtherActor self)
    (`/Game/MMORPG/Core/Common/BpFI_Debug.Debug_Log` (`KismetTextLibrary.Conv_StringToText` (`KismetSystemLibrary.GetObjectName` OtherActor)))))

(fn `Drop`
  (returns (ReturnValue :type "/Game/MMORPG/Items/Weapons/Bp_Weapon Object Reference"))
  (bind _returnvalue (`|SpawnActorFromClass` "/Game/MMORPG/Items/Weapons/Bp_Weapon.Bp_Weapon_C" (`self.GetTransform`) "Undefined" "OverrideRootScale" null "Sword02" null))
  (return _returnvalue))

(fn `UserConstructionScript`
  (set `/Game/MMORPG/Inspect/Bpc_Inspectable.name` (`KismetTextLibrary.Conv_StringToText` (`KismetSystemLibrary.GetObjectName` self)) (`self.Bpc_Inspectable`)))
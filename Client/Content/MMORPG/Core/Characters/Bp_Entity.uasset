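; Bp_Entity is a game entity Blueprint that registers itself with the MMORPG's main game mode.
; On BeginPlay it casts the game mode to Bp_MainGameMode, caches it and adds itself under its EntityID.
; On Destroyed it calls the parent handler, then RemoveGameEntity on the cached game mode, passing a literal 0 instead of its EntityID.
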(event `self.ReceiveBeginPlay`
  (bind _output_get (set `self.GameMode` (cast `/Game/MMORPG/Core/GameMode/Bp_MainGameMode` (`GameplayStatics.GetGameMode`) :!pure true)))
  (`/Engine/EditorBlueprintResources/StandardMacros.IsValid` _output_get
    (:`Is Valid`
      (`/Game/MMORPG/Core/GameMode/Bp_MainGameMode.addGameEntity` (`self.GameMode`) (`self.entityID`) self))))

(event `self.ReceiveDestroyed`
  (bind _gamemode (`self.GameMode`))
  (`parent.ReceiveDestroyed`)
  (`/Engine/EditorBlueprintResources/StandardMacros.IsValid` _gamemode
    (:`Is Valid`
      (`/Game/MMORPG/Core/GameMode/Bp_MainGameMode.removeGameEntity` _gamemode 0))))

(fn `UserConstructionScript`)
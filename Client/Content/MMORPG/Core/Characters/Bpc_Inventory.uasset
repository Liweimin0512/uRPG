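; Inventory component for MMORPG characters that tracks items and equipped gear in two slot maps, ItemSlots and EquipSlots.
; Equip reads the item's slot from its Bpc_Equippable, unequips any different occupant, then equips it on the owning Bp_CharacterBase.
; Equip delegates to the equippable components without writing EquipSlots, which SetEquippedItem updates separately.
; RemoveItem and Unequip are empty stubs.
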(event `self.ReceiveBeginPlay`)

(fn `Equip`
  (params (EquipItem :type "Actor Object Reference"))
  (locals (local_equip :type "Actor Object Reference") (eslot :type "/Game/MMORPG/Characters/EEquipSlot Enum") (oldItem :type "Actor Object Reference"))
  (`/Engine/EditorBlueprintResources/StandardMacros.IsValid` (`Actor.GetComponentByClass` EquipItem "/Game/MMORPG/Core/Item/Bpc_Equippable.Bpc_Equippable_C")
    (:`Is Valid`
      (bind _output_get (set `local.local_equip` EquipItem))
      (bind _output_get_2 (set `local.eslot` (`/Game/MMORPG/Core/Item/Bpc_Equippable.EquipSolt` (`Actor.GetComponentByClass` _output_get "/Game/MMORPG/Core/Item/Bpc_Equippable.Bpc_Equippable_C"))))
      (if true
        (bind _item (`self.GetEquippedItem` _output_get_2))
        (if (!= _item (`local.local_equip`))
          (`/Engine/EditorBlueprintResources/StandardMacros.IsValid` _item
            (:`Is Valid`
              (bind _output_get_3 (set `local.oldItem` _item))
              (bind _asbp_character_base (cast `/Game/MMORPG/Core/Characters/Bp_CharacterBase` (`self.GetOwner`))
                (:`then`
                  (`/Game/MMORPG/Core/Item/Bpc_Equippable.Unequip` (`Actor.GetComponentByClass` _output_get_3 "/Game/MMORPG/Core/Item/Bpc_Equippable.Bpc_Equippable_C") _asbp_character_base))
                (:`CastFailed`
                  (return))))
            (:`Is Not Valid`
              _))
          (bind _asbp_character_base_2 (cast `/Game/MMORPG/Core/Characters/Bp_CharacterBase` (`self.GetOwner`))
            (:`then`
              (`/Game/MMORPG/Core/Item/Bpc_Equippable.Equip` (`Actor.GetComponentByClass` (`local.local_equip`) "/Game/MMORPG/Core/Item/Bpc_Equippable.Bpc_Equippable_C") _asbp_character_base_2)
              (return))
            (:`CastFailed`
              (return)))
          (else
            (return)))
        (else
          (return))))
    (:`Is Not Valid`
      (return))))

(fn `GetEquippedItem`
  (params (EquipType :type "/Game/MMORPG/Characters/EEquipSlot Enum" :default "NewEnumerator13"))
  (returns (item :type "Actor Object Reference"))
  (return (`BlueprintMapLibrary.Map_Find` (`self.EquipSlots`) EquipType)))

(fn `GetItemSlot`
  (params (Item :type "Actor Object Reference"))
  (returns (`Array Element` :type Integer))
  (bind _itemslots (`self.ItemSlots`))
  (bind _keys (`BlueprintMapLibrary.Map_Keys` _itemslots))
  (for _array_element _keys
    (if (== (`BlueprintMapLibrary.Map_Find` _itemslots _array_element) Item)
      (return _array_element))))

(fn `NumItems`
  (returns (ReturnValue :type Integer))
  (return (`BlueprintMapLibrary.Map_Length` (`self.ItemSlots`))))

(fn `RemoveItem`)

(fn `SetEquippedItem`
  (params (Key :type "/Game/MMORPG/Characters/EEquipSlot Enum (by ref)" :default "NewEnumerator13") (Value :type "Actor Object Reference (by ref)"))
  (`BlueprintMapLibrary.Map_Add` (`self.EquipSlots`) Key Value)
  (return))

(fn `Unequip`
  (params (slot :type "/Game/MMORPG/Characters/EEquipSlot Enum" :default "NewEnumerator13")))
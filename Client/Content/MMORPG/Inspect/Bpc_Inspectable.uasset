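; Actor component that makes its owner inspectable, showing its name in the player's main UI widget.
; On BeginPlay it stores the owner's object name as display text.
; Inspect and UnInspect reach the first player controller's main widget to show or clear the inspection, passing the name and a fixed type.
; GetStatus reports "Dead" when the owner's state component says it is dead.
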(event `self.ReceiveBeginPlay`
  (set `self.name` (`KismetTextLibrary.Conv_StringToText` (`KismetSystemLibrary.GetObjectName` (`self.GetOwner`)))))

(event `Inspect`
  (bind _asbp_player_controller (cast `/Game/MMORPG/Core/PlayerController/Bp_PlayerController` (`GameplayStatics.GetPlayerController` 0)))
  (`/Game/MMORPG/Maps/Main/W_Main.Inspect` (`/Game/MMORPG/Core/PlayerController/Bp_PlayerController.W_Main` _asbp_player_controller) (`self.name`) "NewEnumerator1"))

(event `UnInspect`
  (bind _asbp_player_controller (cast `/Game/MMORPG/Core/PlayerController/Bp_PlayerController` (`GameplayStatics.GetPlayerController` 0)))
  (`/Game/MMORPG/Maps/Main/W_Main.UnInspect` (`/Game/MMORPG/Core/PlayerController/Bp_PlayerController.W_Main` _asbp_player_controller)))

(fn `GetStatus`
  (locals (status :type Name))
  (bind _returnvalue (`Actor.GetComponentByClass` (`self.GetOwner`) "/Game/MMORPG/Characters/Common/Bpc_State.Bpc_State_C"))
  (if (and (`KismetSystemLibrary.IsValid` _returnvalue) (`/Game/MMORPG/Characters/Common/Bpc_State.IsDead` _returnvalue))
    (set `local.status` "Dead")))
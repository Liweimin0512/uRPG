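; Game mode for the MMORPG login screen that handles account login and registration through KBEngine.
; On BeginPlay it shows the login widget and mouse cursor and finds the ClientApp actor, whose KBEMain receives login and create-account requests.
; KBEngine result events cast their payload and show error text in the widget, while a successful login opens the avatar selection map.
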(event `self.ReceiveBeginPlay`
  (bind _returnvalue (`|CreateWidget` "/Game/MMORPG/Widgets/UMG_Login.UMG_Login_C"))
  (bind _output_get (set `self.Ref_LoginWidget` _returnvalue))
  (`UserWidget.AddToViewport` _output_get 0)
  (bind _outactors (`GameplayStatics.GetAllActorsOfClass` "/Game/MMORPG/ClientApp.ClientApp_C"))
  (set `self.Ref_ClientApp` (`|GetArrayItem` _outactors))
  (set `PlayerController.bShowMouseCursor` true (`GameplayStatics.GetPlayerController` 0)))

(event `Login`
  (params (username :type String) (password :type String) (datas :type "Array of Byte"))
  (`KBEMain.login` (`/Game/MMORPG/ClientApp.KBEMain` (`self.Ref_ClientApp`)) username password datas))

(event `Register`
  (params (username :type String) (password :type String) (datas :type "Array of Byte (by ref)"))
  (`KBEMain.createAccount` (`/Game/MMORPG/ClientApp.KBEMain` (`self.Ref_ClientApp`)) username password datas))

(event `self.onLoginSuccessfully`
  (params (pEventData :type "KBEventData Object Reference"))
  (`GameplayStatics.OpenLevel` "Map_selectAvatar"))

(event `self.onLoginFailed`
  (params (pEventData :type "KBEventData Object Reference"))
  (bind _askbevent_data_on_login_failed (cast `KBEventData_onLoginFailed` pEventData))
  (`/Game/MMORPG/Widgets/UMG_Login.Error_MSG` (`self.Ref_LoginWidget`) (`KismetTextLibrary.Conv_StringToText` (`KBEventData_onLoginFailed.errorStr` _askbevent_data_on_login_failed))))

(event `self.onReloginBaseappSuccessfully`
  (params (pEventData :type "KBEventData Object Reference"))
  (cast `KBEventData_onReloginBaseappSuccessfully` pEventData)
  (`/Game/MMORPG/Widgets/UMG_Login.Error_MSG` (`self.Ref_LoginWidget`) ""))

(event `self.onLoginBaseappFailed`
  (params (pEventData :type "KBEventData Object Reference"))
  (bind _askbevent_data_on_login_baseapp_failed (cast `KBEventData_onLoginBaseappFailed` pEventData))
  (`/Game/MMORPG/Widgets/UMG_Login.Error_MSG` (`self.Ref_LoginWidget`) (`KismetTextLibrary.Conv_StringToText` (`KBEventData_onLoginBaseappFailed.errorStr` _askbevent_data_on_login_baseapp_failed))))

(event `self.onLoginBaseapp`
  (params (pEventData :type "KBEventData Object Reference"))
  (cast `KBEventData_onLoginBaseapp` pEventData))

(event `self.onCreateAccountResult`
  (params (pEventData :type "KBEventData Object Reference"))
  (bind _askbevent_data_on_create_account_result (cast `KBEventData_onCreateAccountResult` pEventData))
  (`/Game/MMORPG/Widgets/UMG_Login.Error_MSG` (`self.Ref_LoginWidget`) (`KismetTextLibrary.Conv_StringToText` (`KBEventData_onCreateAccountResult.errorStr` _askbevent_data_on_create_account_result))))

(event `self.onKicked`
  (params (pEventData :type "KBEventData Object Reference"))
  (bind _askbevent_data_on_kicked (cast `KBEventData_onKicked` pEventData))
  (`/Game/MMORPG/Widgets/UMG_Login.Error_MSG` (`self.Ref_LoginWidget`) (`KismetTextLibrary.Conv_StringToText` (`KBEventData_onKicked.errorStr` _askbevent_data_on_kicked))))

(event `self.onReloginBaseappFailed`
  (params (pEventData :type "KBEventData Object Reference"))
  (bind _askbevent_data_on_relogin_baseapp_failed (cast `KBEventData_onReloginBaseappFailed` pEventData))
  (`/Game/MMORPG/Widgets/UMG_Login.Error_MSG` (`self.Ref_LoginWidget`) (`KismetTextLibrary.Conv_StringToText` (`KBEventData_onReloginBaseappFailed.errorStr` _askbevent_data_on_relogin_baseapp_failed))))

(fn `UserConstructionScript`)
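; Modular character display actor, apparently the model shown during character selection in an MMORPG.
; On BeginPlay, the face, hair, glove, shoe, headgear, shoulder pad and belt meshes follow the main skeletal mesh through master pose, so one animation drives every part.
; Update takes a character struct, swaps the body and each part mesh, and plays the struct's animation looping on the body.
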(event `self.ReceiveBeginPlay`
  (`SkinnedMeshComponent.SetLeaderPoseComponent` (`self.Hair`) (`self.SkeletalMeshComponent`) false)
  (`SkinnedMeshComponent.SetLeaderPoseComponent` (`self.Glove`) (`self.SkeletalMeshComponent`) false)
  (`SkinnedMeshComponent.SetLeaderPoseComponent` (`self.Shoe`) (`self.SkeletalMeshComponent`) false)
  (`SkinnedMeshComponent.SetLeaderPoseComponent` (`self.HeadGears`) (`self.SkeletalMeshComponent`) false)
  (`SkinnedMeshComponent.SetLeaderPoseComponent` (`self.ShoulderPad`) (`self.SkeletalMeshComponent`) false)
  (`SkinnedMeshComponent.SetLeaderPoseComponent` (`self.Belt`) (`self.SkeletalMeshComponent`) false)
  (`SkinnedMeshComponent.SetLeaderPoseComponent` (`self.Face`) (`self.SkeletalMeshComponent`) false))

(fn `update`
  (params (chapic :type "/Game/MMORPG/Buleprints/Structs/s_chaPic Structure"))
  (bind (`_注释` _model _animtoplay _face _hair _glove _shoe _headgears _shoulderpad _belt) (break `/Game/MMORPG/Buleprints/Structs/s_chaPic` chapic))
  (`SkinnedMeshComponent.SetSkinnedAssetAndUpdate` (`self.SkeletalMeshComponent`) _model true)
  (`SkeletalMeshComponent.PlayAnimation` (`self.SkeletalMeshComponent`) _animtoplay true)
  (`SkinnedMeshComponent.SetSkinnedAssetAndUpdate` (`self.Face`) _face true)
  (`SkinnedMeshComponent.SetSkinnedAssetAndUpdate` (`self.Hair`) _hair true)
  (`SkinnedMeshComponent.SetSkinnedAssetAndUpdate` (`self.Glove`) _glove true)
  (`SkinnedMeshComponent.SetSkinnedAssetAndUpdate` (`self.Shoe`) _shoe true)
  (`SkinnedMeshComponent.SetSkinnedAssetAndUpdate` (`self.HeadGears`) _headgears true)
  (`SkinnedMeshComponent.SetSkinnedAssetAndUpdate` (`self.ShoulderPad`) _shoulderpad true)
  (`SkinnedMeshComponent.SetSkinnedAssetAndUpdate` (`self.Belt`) _belt true))

(fn `UserConstructionScript`)
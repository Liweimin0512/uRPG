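; BP_Building is a clickable MMORPG building that shows an info widget to a nearby player.
; Overlap events track nearby players; releasing a click on the mesh opens W_BuildingInfo with hardcoded tips if the local player is among them, and leaving closes it.
; Cursor hover toggles custom depth on the mesh.
; BeginPlay spawns one hardcoded grocery NPC; the data-driven NPC spawn loop is disconnected, leaving Init empty.
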(event `self.ReceiveBeginPlay`
  (bind _returnvalue (`|SpawnActorFromClass` "/Game/MMORPG/Characters/Npc/Bp_Npc.Bp_Npc_C" (`self.GetTransform`) "AlwaysSpawn" "OverrideRootScale" null "NewEnumerator3" "王老五" null))
  (set `self.Grocery` _returnvalue)
  (`self.init`))

(event `self.ReceiveActorBeginOverlap`
  (params (OtherActor :type "Actor Object Reference"))
  (bind _asbp_player_character (cast `/Game/MMORPG/Characters/Player/BP_PlayerCharacter` OtherActor))
  (`self.AddNearbyPlayer` _asbp_player_character))

(event `self.ReceiveActorEndOverlap`
  (params (OtherActor :type "Actor Object Reference"))
  (bind _asbp_player_character (cast `/Game/MMORPG/Characters/Player/BP_PlayerCharacter` OtherActor))
  (`self.DelNearbyPlayer` _asbp_player_character))

(event `self.StaticMesh.OnReleased`
  (params (TouchedComponent :type "PrimitiveComponent Object Reference") (ButtonReleased :type "Key Structure"))
  (bind _asbp_player_character (cast `/Game/MMORPG/Characters/Player/BP_PlayerCharacter` (`GameplayStatics.GetPlayerCharacter` 0)))
  (if (`KismetArrayLibrary.Array_Contains` (`self.NearbyPlayers`) _asbp_player_character)
    (bind _returnvalue (`|CreateWidget` "/Game/MMORPG/Building/W_BuildingInfo.W_BuildingInfo_C" null (make `/Game/MMORPG/Common/Tips/STips` "北京" "三朝古都" "NewEnumerator1")))
    (bind _output_get (set `/Game/MMORPG/Characters/Player/BP_PlayerCharacter.W_BuildingTips` _returnvalue _asbp_player_character))
    (`UserWidget.AddToViewport` _output_get 0)))

(event `self.StaticMesh.OnBeginCursorOver`
  (params (TouchedComponent :type "PrimitiveComponent Object Reference"))
  (`PrimitiveComponent.SetRenderCustomDepth` (`self.StaticMesh`) true))

(event `self.StaticMesh.OnEndCursorOver`
  (params (TouchedComponent :type "PrimitiveComponent Object Reference"))
  (`PrimitiveComponent.SetRenderCustomDepth` (`self.StaticMesh`) false))

(fn `AddNearbyPlayer`
  (params (NewItem :type "/Game/MMORPG/Characters/Player/BP_PlayerCharacter Object Reference (by ref)"))
  (`KismetArrayLibrary.Array_Add` (`self.NearbyPlayers`) NewItem))

(fn `DelNearbyPlayer`
  (params (Item :type "/Game/MMORPG/Characters/Player/BP_PlayerCharacter Object Reference (by ref)"))
  (bind _w_buildingtips (`/Game/MMORPG/Characters/Player/BP_PlayerCharacter.W_BuildingTips` Item))
  (`KismetArrayLibrary.Array_RemoveItem` (`self.NearbyPlayers`) Item)
  (`/Engine/EditorBlueprintResources/StandardMacros.IsValid` _w_buildingtips
    (:`Is Valid`
      (`/Game/MMORPG/Building/W_BuildingInfo.OnClose_事件_0` _w_buildingtips))))

(fn `init`)

(fn `UserConstructionScript`)
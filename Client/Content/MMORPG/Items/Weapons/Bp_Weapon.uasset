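; Base weapon actor for the MMORPG item system, configured by a weapon ID.
; The construction script looks up that ID in the weapon data table, then sets the static mesh and name from the matching row.
; Equip only returns true, while Unequip destroys the actor and returns true.
; The event graph holds only disabled default events.
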(fn `Equip`
  (returns (`isSuccess?` :type Boolean))
  (return true))

(fn `Unequip`
  (returns (`isSuccess?` :type Boolean))
  (`self.K2_DestroyActor`)
  (return true))

(fn `UserConstructionScript`
  (bind _returnvalue (`|GetDataTableRow` "/Game/MMORPG/Items/Weapons/DT_Weapon.DT_Weapon" (`self.WeaponID`))
    (:`then`
      (bind (_name _meshpic) (break `/Game/MMORPG/Items/Weapons/s_Weapon` _returnvalue))
      (`StaticMeshComponent.SetStaticMesh` (`self.StaticMesh`) _meshpic)
      (set `self.Name` _name))))
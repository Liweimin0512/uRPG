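; Actor component that makes its owning actor an inventory item in the MMORPG item system.
; When put in an inventory, it records the holder, attaches and hides the actor, and fires a callback.
; Removal detaches and unhides it; dropping also repositions the actor and fires a drop callback.
; Helpers expose the holder's inventory component, while pickup, slot lookup and the drop-callback setter are unfinished stubs.
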(event `OnPutInInventory`
  (bind _returnvalue (`self.GetOwner`))
  (`self.SetOwner` null)
  (`Actor.K2_AttachToActor` _returnvalue (`self.owner`) "None" "SnapToTarget" "SnapToTarget" "SnapToTarget" true)
  (`Actor.SetActorHiddenInGame` _returnvalue true)
  (`Actor.K2_SetActorTransform` _returnvalue (`KismetMathLibrary.MakeTransform` (0.0 0.0 0.0)) false false)
  (`self.OnPutinInventoryFn` (`self.owner`)))

(event `OnRemoved`
  (bind _returnvalue (`self.GetOwner`))
  (`/Engine/EditorBlueprintResources/StandardMacros.IsValid` (`self.owner`)
    (:`Is Valid`
      (`Actor.K2_DetachFromActor` _returnvalue "KeepRelative" "KeepRelative" "KeepRelative")
      (`self.ClearOwner`)
      (`Actor.SetActorHiddenInGame` _returnvalue false))))

(event `OnDropped`
  (bind _returnvalue (`self.GetOwner`))
  (bind _owner (`self.owner`))
  (`/Engine/EditorBlueprintResources/StandardMacros.IsValid` _returnvalue
    (:`Is Valid`
      (`self.OnRemoved`)
      (`Actor.K2_SetActorLocation` (`self.GetOwner`) (select `bool` (`KismetSystemLibrary.IsValid` _owner) :`false` (`Actor.K2_GetActorLocation` _returnvalue) :`true` (`Actor.K2_GetActorLocation` _owner)) false false)
      (`self.OnDropFn`))))

(event `OnPickup`)

(fn `ClearOwner`
  (set `self.owner` null)
  (return))

(fn `GetContainer`
  (returns (Bpc_Inventory :type "/Game/MMORPG/Characters/Common/Bpc_Inventory Object Reference"))
  (bind _owner (`self.owner`))
  (`/Engine/EditorBlueprintResources/StandardMacros.IsValid` _owner
    (:`Is Valid`
      (return (`/Game/MMORPG/Core/Characters/Bp_Entity.Bpc_Inventory` _owner)))))

(fn `GetDebugString`
  (returns (Image :type Text))
  (return (`|FormatText` "inventory image name set to:{imagename}" (`KismetTextLibrary.Conv_NameToText` (`self.imageName`)))))

(fn `GetSlotNum`
  (locals (ct :type "/Game/MMORPG/Characters/Common/Bpc_Inventory Object Reference"))
  (bind _owner (`self.owner`))
  (`/Engine/EditorBlueprintResources/StandardMacros.IsValid` _owner
    (:`Is Valid`
      (bind _output_get (set `local.ct` (`/Game/MMORPG/Core/Characters/Bp_Entity.Bpc_Inventory` _owner)))
      (`/Engine/EditorBlueprintResources/StandardMacros.IsValid` _output_get
        (:`Is Valid`
          (return))))))

(fn `SetOnActiveItemFn`
  (params (fn :type Name))
  (set `self.onActiveitemFn` fn)
  (return))

(fn `SetOnDroppedFn`
  (params (fn :type Name)))

(fn `SetOwner`
  (params (owner :type "/Game/MMORPG/Core/Characters/Bp_Entity Object Reference"))
  (set `self.owner` owner)
  (return))
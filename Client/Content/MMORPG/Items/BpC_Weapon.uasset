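; Weapon component that gives its owning actor melee hit detection and basic ranged-attack support, storing damage, range and projectile settings.
; It binds to the owner's overlap event and calls OnHit on the other actor's Bpc_Combat when OwnerEntity's combat component flags both IsHit and IsAttack.
; LaunchProjectile fires a launch dispatcher and spawns the projectile's class at the world origin, while CanRangedAttack is a TODO that always returns true.
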(event `self.ReceiveBeginPlay`
  (bind _returnvalue (`self.GetOwner`))
  (`|ExecutionSequence`
    (:`then_2`
      (`/Engine/EditorBlueprintResources/StandardMacros.IsValid` _returnvalue
        (:`Is Valid`
          (add `Actor.OnActorBeginOverlap` _returnvalue (delegate `OnActorBeginOverlap_事件_0`)))))))

(event `OnActorBeginOverlap_事件_0`
  (params (OverlappedActor :type "Actor Object Reference") (OtherActor :type "Actor Object Reference"))
  (bind _returnvalue (`Actor.GetComponentByClass` OtherActor "/Game/MMORPG/Characters/Common/Bpc_Combat.Bpc_Combat_C"))
  (bind _ownerentity (`self.ownerEntity`))
  (`/Engine/EditorBlueprintResources/StandardMacros.IsValid` _ownerentity
    (:`Is Valid`
      (if (and (!= OtherActor _ownerentity) (`/Game/MMORPG/Characters/Common/Bpc_Combat.isHit?` (`Actor.GetComponentByClass` _ownerentity "/Game/MMORPG/Characters/Common/Bpc_Combat.Bpc_Combat_C")))
        (if (`/Game/MMORPG/Characters/Common/Bpc_Combat.isAttack?` (`Actor.GetComponentByClass` _ownerentity "/Game/MMORPG/Characters/Common/Bpc_Combat.Bpc_Combat_C"))
          (`/Engine/EditorBlueprintResources/StandardMacros.IsValid` _returnvalue
            (:`Is Valid`
              (`/Game/MMORPG/Characters/Common/Bpc_Combat.OnHit` _returnvalue null (`self.GetOwner`)))
            (:`Is Not Valid`
              (`KismetSystemLibrary.PrintString` "hiter has no combat component"))))
        (else
          (`KismetSystemLibrary.PrintString` "is not attack"))))))

(event `self.ReceiveEndPlay`
  (params (EndPlayReason :type "EEndPlayReason Enum" :default "Destroyed"))
  (remove `Actor.OnActorBeginOverlap` (`self.GetOwner`) (delegate `OnActorBeginOverlap_事件_0`)))

(fn `CanRangedAttack`
  (returns (canRangedAttack :type Boolean))
  (return true))

(fn `LaunchProjectile`
  (params (attacker :type "Actor Object Reference") (target :type "Actor Object Reference"))
  (locals (proj :type "Actor Object Reference"))
  (bind _projectile (`self.projectile`))
  (`/Engine/EditorBlueprintResources/StandardMacros.IsValid` _projectile
    (:`Is Valid`
      (`self.onprojectilelaunchfn` attacker target)
      (`|SpawnActorFromClass` (`GameplayStatics.GetObjectClass` _projectile) (`KismetMathLibrary.MakeTransform` (0.0 0.0 0.0)) "Undefined" "OverrideRootScale" null null))))

(fn `SetDamage`
  (params (damage :type Integer))
  (set `self.damage` damage)
  (return))

(fn `SetProjectile`
  (params (projectile :type "Actor Object Reference"))
  (set `self.projectile` projectile))

(fn `SetRange`
  (params (attackrange :type Integer) (hitrange :type Integer))
  (set `self.attackrange` attackrange)
  (set `self.hitrange` hitrange)
  (return))
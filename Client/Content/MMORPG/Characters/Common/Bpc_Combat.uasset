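; Combat component for a Bp_Entity owner, handling attacks, damage taken and weapon changes.
; Attack broadcasts the weapon type and plays a fixed montage, with flags blocking re-entry.
; OnHit applies fixed damage to the owner, whose damage handler plays a hit montage and lowers a Bpc_State stat.
; WeaponChange reads DT_Weapon, unequips by holding method, then spawns and socket-attaches the new weapon, but sets its slot variable to None.
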(event `self.ReceiveBeginPlay`
  (add `Actor.OnTakeAnyDamage` (`self.GetOwner`) (delegate `OnTakeAnyDamage_事件_0`)))

(event `OnTakeAnyDamage_事件_0`
  (params (DamagedActor :type "Actor Object Reference") (Damage :type "Float (double-precision)") (DamageType :type "DamageType Object Reference") (InstigatedBy :type "Controller Object Reference") (DamageCauser :type "Actor Object Reference"))
  (bind _returnvalue (`self.GetOwner`))
  (bind _returnvalue_2 (`Actor.GetComponentByClass` _returnvalue "/Game/MMORPG/Characters/Common/Bpc_State.Bpc_State_C"))
  (`|PlayMontage` (`Character.Mesh` (cast `/Game/MMORPG/Core/Characters/Bp_Entity` _returnvalue :!pure true)) "/Game/MMORPG/Characters/Common/Animations/GetHit_BowAnim_Montage.GetHit_BowAnim_Montage"
    (:`then`
      (`/Engine/EditorBlueprintResources/StandardMacros.IsValid` _returnvalue_2
        (:`Is Valid`
          (`/Game/MMORPG/Characters/Common/Bpc_State.ModifyStat` _returnvalue_2 "NewEnumerator1" (* (`KismetMathLibrary.FTrunc` Damage) -1)))))))

(event `self.ReceiveEndPlay`
  (params (EndPlayReason :type "EEndPlayReason Enum" :default "Destroyed"))
  (remove `Actor.OnTakeAnyDamage` (`self.GetOwner`) (delegate `OnTakeAnyDamage_事件_0`)))

(event `Attack`
  (bind _weapontype (`self.WeaponType`))
  (bind (_asbp_entity _bsuccess) (cast `/Game/MMORPG/Core/Characters/Bp_Entity` (`self.GetOwner`) :!pure true))
  (if (`|EnumInequality` _weapontype "NewEnumerator5")
    (if (and _bsuccess (not (`self.isAttack?`)))
      (`self.OnAttack` _weapontype)
      (set `self.isAttack?` true)
      (set `self.isHit?` true)
      (`|PlayMontage` (`Character.Mesh` _asbp_entity) "/Game/MMORPG/Characters/Common/Animations/NormalAttack01_DoubleSwordAnim_Montage.NormalAttack01_DoubleSwordAnim_Montage"
        (:`OnCompleted`
          (set `self.isAttack?` false)
          (set `self.isHit?` false))))))

(event `WeaponChange`
  (params (WeaponID :type Name))
  (bind _returnvalue (`self.GetOwner`))
  (bind _leftweapon (`self.LeftWeapon`))
  (bind _rightweapon (`self.RightWeapon`))
  (bind _returnvalue_2 (`|GetDataTableRow` "/Game/MMORPG/Items/Weapons/DT_Weapon.DT_Weapon" WeaponID)
    (:`then`
      (bind ((`WeaponType_14_6EEC250A4E7AE9B723CD5EB1C16F5062` _weapontype) (`HoldingMethod_18_B43486B040DCC8FF2E0D09838581B904` _holdingmethod)) (break `/Game/MMORPG/Items/Weapons/s_Weapon` _returnvalue_2))
      (switch `/Game/MMORPG/Items/Weapons/EHoldingMethod` _holdingmethod
        (:`NewEnumerator0`
          (`/Engine/EditorBlueprintResources/StandardMacros.IsValid` _leftweapon
            (:`Is Valid`
              (bind _issuccess_ (`/Game/MMORPG/Items/Weapons/Bp_Weapon.Unequip` _leftweapon))
              (if _issuccess_
                (bind _returnvalue_3 (`|SpawnActorFromClass` "/Game/MMORPG/Items/Weapons/Bp_Weapon.Bp_Weapon_C" (`Actor.GetTransform` _returnvalue) "Undefined" "OverrideRootScale" null WeaponID null :!label _label))
                (bind _asbp_player_character (cast `/Game/MMORPG/Characters/Player/BP_PlayerCharacter` _returnvalue))
                (`Actor.K2_AttachToComponent` _returnvalue_3 (`Character.Mesh` _asbp_player_character) (select `/Game/MMORPG/Items/Weapons/EHoldingMethod` _holdingmethod :`NewEnumerator0` "LeftWeaponShield" :`NewEnumerator1` "RightWeaponShield" :`NewEnumerator2` "RightWeaponShield" :!type "Name") "SnapToTarget" "SnapToTarget" "SnapToTarget" true)
                (set `/Game/MMORPG/Items/BpC_Weapon.ownerEntity` (cast `/Game/MMORPG/Core/Characters/Bp_Entity` (`self.GetOwner`) :!pure true) (`Actor.GetComponentByClass` _returnvalue_3 "/Game/MMORPG/Items/BpC_Weapon.Bpc_Weapon_C"))
                (`/Game/MMORPG/Items/Weapons/Bp_Weapon.Equip` _returnvalue_3)
                (switch `/Game/MMORPG/Items/Weapons/EHoldingMethod` _holdingmethod
                  (:`NewEnumerator0`
                    (set `self.LeftWeapon` null))
                  (:`NewEnumerator1`
                    (set `self.RightWeapon` null :!label _label_2))
                  (:`NewEnumerator2`
                    (goto _label_2)))
                (set `self.WeaponType` _weapontype)))
            (:`Is Not Valid`
              (goto _label))))
        (:`NewEnumerator1`
          (`/Engine/EditorBlueprintResources/StandardMacros.IsValid` _rightweapon
            (:`Is Valid`
              (bind _issuccess__2 (`/Game/MMORPG/Items/Weapons/Bp_Weapon.Unequip` _rightweapon))
              (if _issuccess__2
                (goto _label)))
            (:`Is Not Valid`
              (goto _label))))
        (:`NewEnumerator2`
          (`/Engine/EditorBlueprintResources/StandardMacros.IsValid` (`self.LeftWeapon`)
            (:`Is Valid`
              (bind _issuccess__3 (`/Game/MMORPG/Items/Weapons/Bp_Weapon.Unequip` (`self.LeftWeapon`))))
            (:`Is Not Valid`
              _))
          (`/Engine/EditorBlueprintResources/StandardMacros.IsValid` (`self.RightWeapon`)
            (:`Is Valid`
              (bind _issuccess__4 (`/Game/MMORPG/Items/Weapons/Bp_Weapon.Unequip` (`self.RightWeapon`)))
              (if (and _issuccess__3 _issuccess__4)
                (goto _label)))
            (:`Is Not Valid`
              (goto _label))))))
    (:`RowNotFound`
      (`KismetSystemLibrary.PrintString` (`KismetTextLibrary.Conv_TextToString` (`|FormatText` "无法找到指定的武器{weapon}" (`KismetTextLibrary.Conv_NameToText` WeaponID)))))))

(event `OnHit`
  (params (instigator :type "Controller Object Reference") (Causer :type "Actor Object Reference"))
  (set `self.isHit?` false)
  (`GameplayStatics.ApplyDamage` (`self.GetOwner`) 10.0 instigator Causer))
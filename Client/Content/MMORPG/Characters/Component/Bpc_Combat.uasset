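; Combat component that handles attack requests and weapon swapping for the owning player character.
; Attack fires the OnAttack dispatcher unless WeaponType is one excluded enum value.
; WeaponChange looks up the ID in DT_Weapon and unequips weapons conflicting with its holding method.
; It then spawns a Bp_Weapon, snaps it to a hand socket on the character mesh and stores it as LeftWeapon or RightWeapon, two-handed using the right.
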(event `self.ReceiveBeginPlay`)

(event `self.ReceiveTick`
  (params (DeltaSeconds :type "Float (single-precision)")))

(event `Attack`
  (if (`|EnumInequality` (`self.WeaponType`) "NewEnumerator5")
    (`self.OnAttack`)))

(event `WeaponChange`
  (params (WeaponID :type Name))
  (bind _returnvalue (`self.GetOwner`))
  (bind _leftweapon (`self.LeftWeapon`))
  (bind _rightweapon (`self.RightWeapon`))
  (bind _returnvalue_2 (`|GetDataTableRow` "/Game/MMORPG/Items/Weapons/DT_Weapon.DT_Weapon" WeaponID)
    (:`then`
      (bind ((`HoldingMethod_18_B43486B040DCC8FF2E0D09838581B904` _holdingmethod)) (break `/Game/MMORPG/Items/Weapons/s_Weapon` _returnvalue_2))
      (switch `/Game/MMORPG/Items/Weapons/EHoldingMethod` _holdingmethod
        (:`NewEnumerator0`
          (`/Engine/EditorBlueprintResources/StandardMacros.IsValid` _leftweapon
            (:`Is Valid`
              (bind _issuccess_ (`/Game/MMORPG/Items/Weapons/Bp_Weapon.Unequip` _leftweapon))
              (if _issuccess_
                (bind _returnvalue_3 (`|SpawnActorFromClass` "/Game/MMORPG/Items/Weapons/Bp_Weapon.Bp_Weapon_C" (`Actor.GetTransform` _returnvalue) "Undefined" "OverrideRootScale" null WeaponID null :!label _label))
                (bind _asbp_player_character (cast `/Game/MMORPG/Characters/Player/BP_PlayerCharacter` _returnvalue))
                (`Actor.K2_AttachToComponent` _returnvalue_3 (`Character.Mesh` _asbp_player_character) (select `/Game/MMORPG/Items/Weapons/EHoldingMethod` _holdingmethod :`NewEnumerator0` "LeftWeaponShield" :`NewEnumerator1` "RightWeaponShield" :`NewEnumerator2` "RightWeaponShield" :!type "Name") "SnapToTarget" "SnapToTarget" "SnapToTarget" true)
                (`/Game/MMORPG/Items/Weapons/Bp_Weapon.Equip` _returnvalue_3)
                (switch `/Game/MMORPG/Items/Weapons/EHoldingMethod` _holdingmethod
                  (:`NewEnumerator0`
                    (set `self.LeftWeapon` _returnvalue_3))
                  (:`NewEnumerator1`
                    (set `self.RightWeapon` _returnvalue_3 :!label _label_2))
                  (:`NewEnumerator2`
                    (goto _label_2)))))
            (:`Is Not Valid`
              (goto _label))))
        (:`NewEnumerator1`
          (`/Engine/EditorBlueprintResources/StandardMacros.IsValid` _rightweapon
            (:`Is Valid`
              (bind _issuccess__2 (`/Game/MMORPG/Items/Weapons/Bp_Weapon.Unequip` _rightweapon))
              (if _issuccess__2
                (goto _label)))
            (:`Is Not Valid`
              (goto _label))))
        (:`NewEnumerator2`
          (`/Engine/EditorBlueprintResources/StandardMacros.IsValid` (`self.LeftWeapon`)
            (:`Is Valid`
              (bind _issuccess__3 (`/Game/MMORPG/Items/Weapons/Bp_Weapon.Unequip` (`self.LeftWeapon`))))
            (:`Is Not Valid`
              _))
          (`/Engine/EditorBlueprintResources/StandardMacros.IsValid` (`self.RightWeapon`)
            (:`Is Valid`
              (bind _issuccess__4 (`/Game/MMORPG/Items/Weapons/Bp_Weapon.Unequip` (`self.RightWeapon`)))
              (if (and _issuccess__3 _issuccess__4)
                (goto _label)))
            (:`Is Not Valid`
              (goto _label))))))
    (:`RowNotFound`
      (`KismetSystemLibrary.PrintString` (`KismetTextLibrary.Conv_TextToString` (`|FormatText` "无法找到指定的武器{weapon}" (`KismetTextLibrary.Conv_NameToText` WeaponID)))))))
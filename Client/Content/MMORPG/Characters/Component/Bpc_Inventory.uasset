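; Inventory actor component that stores items in an ItemSlots map from slot index to item data.
; AddItem looks up the ItemID row in DT_Item and stores it at the first free index below MaxSlots.
; GetNullSlots returns -1 when every slot is full, and AddItem adds at that key without checking.
; NumItems returns the map size; SelectActiveItemFromSlot is an empty stub.
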(fn `AddItem`
  (params (ItemID :type Name))
  (bind _returnvalue (`|GetDataTableRow` "/Game/MMORPG/Items/DT_Item.DT_Item" ItemID)
    (:`then`
      (bind _index (`self.getNullSlots`))
      (`BlueprintMapLibrary.Map_Add` (`self.ItemSlots`) _index _returnvalue))))

(fn `getNullSlots`
  (returns (Index :type Integer))
  (for _index (range (`self.maxSlots`))
    (if (not (`.ReturnValue` (`BlueprintMapLibrary.Map_Find` (`self.ItemSlots`) _index)))
      (return _index)))
  (return -1))

(fn `NumItems`
  (returns (num :type Integer))
  (return (`BlueprintMapLibrary.Map_Length` (`self.ItemSlots`))))

(fn `SelectActiveItemFromSlot`
  (params (slot :type Integer))
  (locals (OldItem :type "/Game/MMORPG/Items/SItem Structure") (NewItem :type "/Game/MMORPG/Items/SItem Structure")))
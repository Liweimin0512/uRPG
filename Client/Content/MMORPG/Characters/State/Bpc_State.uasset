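; Character state component for the MMORPG that holds stats in a map keyed by stat type.
; GetState and SetState read and write entries, while ModifyStat adds a delta to the current value, clamps it to that stat's range and stores it.
; Each change fires the OnSateModifiy dispatcher, then OnDead whenever one designated stat, presumably health, sits at its minimum, even if another stat changed.
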(fn `GetState`
  (params (Key :type "/Game/MMORPG/Characters/State/EStat Enum" :default "NewEnumerator0"))
  (returns (Value :type "/Game/MMORPG/Characters/State/SStat Structure"))
  (return (`BlueprintMapLibrary.Map_Find` (`self.StatData`) Key)))

(fn `IsDead`
  (returns (`isDead?` :type Boolean))
  (bind ((`MinValue_2_A1EE3CBC4EBEB0911189BEBFA4142BF3` _minvalue) (`CurrentValue_6_732DC4904498B7F1B40268AAFBBD2BF4` _currentvalue)) (break `/Game/MMORPG/Characters/State/SStat` (`self.GetState` "NewEnumerator1")))
  (return (== _minvalue _currentvalue)))

(fn `ModifyStat`
  (params (Key :type "/Game/MMORPG/Characters/State/EStat Enum" :default "NewEnumerator0") (By :type Integer))
  (bind _value (`self.GetState` Key))
  (bind (_minvalue _maxvalue _currentvalue) (break `/Game/MMORPG/Characters/State/SStat` _value))
  (bind _structout (setmembers `/Game/MMORPG/Characters/State/SStat` :`StructRef` _value :`CurrentValue` (`KismetMathLibrary.Clamp` (+ _currentvalue By) _minvalue _maxvalue)))
  (`self.SetState` Key _structout)
  (`self.OnSateModifiy` Key _structout)
  (if (`self.IsDead`)
    (`self.OnDead`)
    (return)
    (else
      (return))))

(fn `SetState`
  (params (Key :type "/Game/MMORPG/Characters/State/EStat Enum" :default "NewEnumerator0") (Value :type "/Game/MMORPG/Characters/State/SStat Structure (by ref)"))
  (`BlueprintMapLibrary.Map_Add` (`self.StatData`) Key Value)
  (return))
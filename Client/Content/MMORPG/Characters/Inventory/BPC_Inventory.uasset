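; Inventory component for an MMORPG character, holding carried item stacks and a slot-to-item map of equipment.
; Equip and Unequip delegate to each item's Bpc_Equippable, swapping out the slot's occupant, and require a Bp_CharacterBase owner.
; GiveItem merges one unit into a matching stack using DT_Item's stack limit, splitting overflow, then fires a notification.
; Equipment queries cover gameplay tags and slots; remove, drop, use and delete are empty stubs.
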(event `self.ReceiveBeginPlay`)

(fn `DeleteItem`)

(fn `DropItem`
  (params (Item :type "Actor Object Reference") (pos :type "Vector Structure")))

(fn `Equip`
  (params (EquipItem :type "Actor Object Reference"))
  (locals (local_equip :type "Actor Object Reference") (eslot :type "/Game/MMORPG/Characters/EEquipSlot Enum") (oldItem :type "Actor Object Reference"))
  (`/Engine/EditorBlueprintResources/StandardMacros.IsValid` (`Actor.GetComponentByClass` EquipItem "/Game/MMORPG/Core/Item/Bpc_Equippable.Bpc_Equippable_C")
    (:`Is Valid`
      (bind _output_get (set `local.local_equip` EquipItem))
      (bind _output_get_2 (set `local.eslot` (`/Game/MMORPG/Core/Item/Bpc_Equippable.EquipSolt` (`Actor.GetComponentByClass` _output_get "/Game/MMORPG/Core/Item/Bpc_Equippable.Bpc_Equippable_C"))))
      (if true
        (bind _item (`self.GetEquippedItem` _output_get_2))
        (if (!= _item (`local.local_equip`))
          (`/Engine/EditorBlueprintResources/StandardMacros.IsValid` _item
            (:`Is Valid`
              (bind _output_get_3 (set `local.oldItem` _item))
              (bind _asbp_character_base (cast `/Game/MMORPG/Core/Characters/Bp_CharacterBase` (`self.GetOwner`))
                (:`then`
                  (`/Game/MMORPG/Core/Item/Bpc_Equippable.Unequip` (`Actor.GetComponentByClass` _output_get_3 "/Game/MMORPG/Core/Item/Bpc_Equippable.Bpc_Equippable_C") _asbp_character_base))
                (:`CastFailed`
                  (return))))
            (:`Is Not Valid`
              _))
          (bind _asbp_character_base_2 (cast `/Game/MMORPG/Core/Characters/Bp_CharacterBase` (`self.GetOwner`))
            (:`then`
              (`/Game/MMORPG/Core/Item/Bpc_Equippable.Equip` (`Actor.GetComponentByClass` (`local.local_equip`) "/Game/MMORPG/Core/Item/Bpc_Equippable.Bpc_Equippable_C") _asbp_character_base_2)
              (return))
            (:`CastFailed`
              (return)))
          (else
            (return)))
        (else
          (return))))
    (:`Is Not Valid`
      (return))))

(fn `EquipHasTag`
  (params (Tag :type "GameplayTag Structure"))
  (returns (ReturnValue :type Boolean))
  (bind _values (`self.GetAllEquips`))
  (for _array_element _values
    (bind _returnvalue (message `GameplayTagAssetInterface.HasMatchingGameplayTag` _array_element Tag))
    (if _returnvalue
      (return true)))
  (return false))

(fn `GetAllEquips`
  (returns (Values :type "Array of Actor Object Reference"))
  (bind _values (`BlueprintMapLibrary.Map_Values` (`self.EquipSlots`)))
  (return _values))

(fn `GetEquippedItem`
  (params (EquipType :type "/Game/MMORPG/Characters/EEquipSlot Enum" :default "NewEnumerator13"))
  (returns (item :type "Actor Object Reference"))
  (return (`BlueprintMapLibrary.Map_Find` (`self.EquipSlots`) EquipType)))

(fn `GetItem`
  (params (Key :type "Integer (by ref)"))
  (returns (Output :type "/Game/MMORPG/Items/SCurrentItem Structure"))
  (return (`|GetArrayItem` (`self.Item`) Key)))

(fn `GiveItem`
  (params (Item :type "/Game/MMORPG/Items/SCurrentItem Structure"))
  (locals (StackLimit :type Integer) (CurrentItem :type "/Game/MMORPG/Items/SCurrentItem Structure") (NewItem :type "/Game/MMORPG/Items/SCurrentItem Structure"))
  (bind _newitem (`local.NewItem`))
  (bind ((`ItemID_2_AC19A79446DCDA6515B1E1A1FBF22B06` _itemid)) (break `/Game/MMORPG/Items/SCurrentItem` (`local.NewItem`)))
  (bind _output_get (set `local.NewItem` Item))
  (bind _returnvalue (`|GetDataTableRow` "/Game/MMORPG/Items/DT_Item.DT_Item" (`.ItemID_2_AC19A79446DCDA6515B1E1A1FBF22B06` (break `/Game/MMORPG/Items/SCurrentItem` _output_get)))
    (:`then`
      (bind (_name _type _stacklimit) (break `/Game/MMORPG/Items/SItem` _returnvalue))
      (set `local.StackLimit` _stacklimit)
      (if (!= _stacklimit 0)
        (for _array_element (`self.Item`)
          (set `local.CurrentItem` _array_element)
          (bind (_itemid_2 _itemcount) (break `/Game/MMORPG/Items/SCurrentItem` _array_element))
          (if (== _itemid_2 (`.ItemID_2_AC19A79446DCDA6515B1E1A1FBF22B06` (break `/Game/MMORPG/Items/SCurrentItem` (`local.NewItem`))))
            (bind _returnvalue_2 (+ _itemcount 1))
            (if (<= _returnvalue_2 (`local.StackLimit`))
              (`KismetArrayLibrary.Array_Add` (`self.Item`) (make `/Game/MMORPG/Items/SCurrentItem` (`.ItemID_2_AC19A79446DCDA6515B1E1A1FBF22B06` (break `/Game/MMORPG/Items/SCurrentItem` (`local.NewItem`))) _returnvalue_2))
              (`KismetArrayLibrary.Array_RemoveItem` (`self.Item`) (`local.CurrentItem`))
              (`self.OnGiveItem` (`local.NewItem`))
              (return)
              (else
                (`KismetArrayLibrary.Array_Add` (`self.Item`) (make `/Game/MMORPG/Items/SCurrentItem` _itemid (- _returnvalue_2 (`local.StackLimit`))))
                (`KismetArrayLibrary.Array_Add` (`self.Item`) (make `/Game/MMORPG/Items/SCurrentItem` _itemid (`local.StackLimit`)))
                (`KismetArrayLibrary.Array_RemoveItem` (`self.Item`) (`local.CurrentItem`))
                (`self.OnGiveItem` (`local.NewItem`))
                (return))))))
      (`KismetArrayLibrary.Array_Add` (`self.Item`) _newitem)
      (`self.OnGiveItem` _newitem)
      (return))))

(fn `isItemEquipped`
  (params (Item :type "Actor Object Reference"))
  (returns (Output :type "/Game/MMORPG/Characters/EEquipSlot Enum"))
  (bind _values (`self.GetAllEquips`))
  (for (_array_element _array_index) _values
    (if (== _array_element Item)
      (bind _keys (`BlueprintMapLibrary.Map_Keys` (`self.EquipSlots`)))
      (return (`|GetArrayItem` _keys _array_index)))))

(fn `RemoveItem`)

(fn `RemoveItemBySlot`
  (params (Slot :type Integer :default 0)))

(fn `SetEquippedItem`
  (params (Key :type "/Game/MMORPG/Characters/EEquipSlot Enum (by ref)" :default "NewEnumerator13") (Value :type "Actor Object Reference"))
  (`BlueprintMapLibrary.Map_Add` (`self.EquipSlots`) Key Value)
  (return))

(fn `SetItem`)

(fn `Unequip`
  (params (slot :type "/Game/MMORPG/Characters/EEquipSlot Enum" :default "NewEnumerator13"))
  (locals (LocalItem :type "Actor Object Reference"))
  (bind _returnvalue (`Actor.GetComponentByClass` (`local.LocalItem`) "/Game/MMORPG/Core/Item/Bpc_Equippable.Bpc_Equippable_C"))
  (bind _output_get (set `local.LocalItem` (`self.GetEquippedItem` slot)))
  (`/Engine/EditorBlueprintResources/StandardMacros.IsValid` _output_get
    (:`Is Valid`
      (`/Engine/EditorBlueprintResources/StandardMacros.IsValid` _returnvalue
        (:`Is Valid`
          (bind _asbp_character_base (cast `/Game/MMORPG/Core/Characters/Bp_CharacterBase` (`self.GetOwner`))
            (:`then`
              (`/Game/MMORPG/Core/Item/Bpc_Equippable.Unequip` _returnvalue _asbp_character_base))
            (:`CastFailed`
              (`/Game/MMORPG/Core/Common/BpFI_Debug.Debug_Error` "Item Owner is not CharacterBase!!!")
              (return))))
        (:`Is Not Valid`
          _))
      (`self.SetEquippedItem` slot)
      (`self.OnUnequip` (`local.LocalItem`) slot)
      (return))))

(fn `UseItemFromInvTile`
  (params (Item :type "Actor Object Reference")))
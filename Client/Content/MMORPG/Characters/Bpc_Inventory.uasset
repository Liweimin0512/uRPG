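; Inventory component for MMORPG characters that exposes queries over the items held in its ItemSlots map.
; GetItemSlot does a reverse lookup by scanning the map's keys for the first slot holding the given item, and NumItems returns the map's entry count.
; GetEquippedItem takes an equip type but is an empty stub, and the component's BeginPlay and Tick events contain no logic.
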(event `self.ReceiveBeginPlay`)

(fn `GetEquippedItem`
  (params (EquipType :type "/Game/MMORPG/Characters/EEquipSlot Enum" :default "NewEnumerator13"))
  (returns (item :type "Actor Object Reference"))
  (return null))

(fn `GetItemSlot`
  (params (Item :type "Actor Object Reference"))
  (returns (`Array Element` :type Integer))
  (bind _itemslots (`self.ItemSlots`))
  (bind _keys (`BlueprintMapLibrary.Map_Keys` _itemslots))
  (for _array_element _keys
    (if (== (`BlueprintMapLibrary.Map_Find` _itemslots _array_element) Item)
      (return _array_element))))

(fn `NumItems`
  (returns (ReturnValue :type Integer))
  (return (`BlueprintMapLibrary.Map_Length` (`self.ItemSlots`))))